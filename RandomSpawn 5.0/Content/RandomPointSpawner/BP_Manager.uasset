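; Level manager that, on BeginPlay, moves four existing actors (cube, cylinder, sphere, cone) to four spawn point actors in random order, one per point.
; Each actor has its own event with a staggered Delay, finding the actor and points by class and using Teleport instead of spawning.
; A random, non-looping MultiGate picks a point and re-enters itself when that point's shared Active flag is already set, preventing overlaps.
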(event `self.ReceiveBeginPlay`
  ;[1 1 1] Call Actor Spawns At Level Load
  (`|ExecutionSequence`
    (:`then_0`
      (`self.SpawnActor1`))
    (:`then_1`
      (`self.SpawnActor2`))
    (:`then_2`
      (`self.SpawnActor3`))
    (:`then_3`
      (`self.SpawnActor4`))))

(event `SpawnActor3`
  ;[1 1 1] Spawn Actor 3
  (`KismetSystemLibrary.Delay` 0.8)
  (if (not (`self.Actor3Active`))
    (bind _asbp_sphere (castclass `/Game/RandomPointSpawner/Actors/BP_Sphere` "/Game/RandomPointSpawner/Actors/BP_Sphere.BP_Sphere_C"))
    (bind _returnvalue (`GameplayStatics.GetActorOfClass` _asbp_sphere))
    (`|MultiGate` true :!label _label ; Spawn At Random Point
      (:`Out 0`
        (if (`self.SpawnPoint1Active`)
          (goto _label)
          (else
            (set `self.SpawnPoint1Active` true) ; Set Spawn Point As Active (Used)
            (bind _asbp_spawn_point_1 (castclass `/Game/RandomPointSpawner/SpawnPoints/BP_SpawnPoint1` "/Game/RandomPointSpawner/SpawnPoints/BP_SpawnPoint1.BP_SpawnPoint1_C"))
            (bind _returnvalue_2 (`GameplayStatics.GetActorOfClass` _asbp_spawn_point_1))
            (`self.K2_TeleportTo` :`self` _returnvalue :`DestLocation` (`self.K2_GetActorLocation` _returnvalue_2)) ; Spawn Point 1
          )))
      (:`Out 1`
        (if (`self.SpawnPoint2Active`)
          (goto _label)
          (else
            (set `self.SpawnPoint2Active` true)
            (bind _asbp_spawn_point_2 (castclass `/Game/RandomPointSpawner/SpawnPoints/BP_SpawnPoint2` "/Game/RandomPointSpawner/SpawnPoints/BP_SpawnPoint2.BP_SpawnPoint2_C"))
            (bind _returnvalue_3 (`GameplayStatics.GetActorOfClass` _asbp_spawn_point_2))
            (`self.K2_TeleportTo` :`self` _returnvalue :`DestLocation` (`self.K2_GetActorLocation` _returnvalue_3)) ; Spawn Point 2
          )))
      (:`Out 2`
        (if (`self.SpawnPoint3Active`)
          (goto _label)
          (else
            (set `self.SpawnPoint3Active` true)
            (bind _asbp_spawn_point_3 (castclass `/Game/RandomPointSpawner/SpawnPoints/BP_SpawnPoint3` "/Game/RandomPointSpawner/SpawnPoints/BP_SpawnPoint3.BP_SpawnPoint3_C"))
            (bind _returnvalue_4 (`GameplayStatics.GetActorOfClass` _asbp_spawn_point_3))
            (`self.K2_TeleportTo` :`self` _returnvalue :`DestLocation` (`self.K2_GetActorLocation` _returnvalue_4)) ; Spawn Point 3
          )))
      (:`Out 3`
        (if (`self.SpawnPoint4Active`)
          (goto _label)
          (else
            (set `self.SpawnPoint4Active` true)
            (bind _asbp_spawn_point_4 (castclass `/Game/RandomPointSpawner/SpawnPoints/BP_SpawnPoint4` "/Game/RandomPointSpawner/SpawnPoints/BP_SpawnPoint4.BP_SpawnPoint4_C"))
            (bind _returnvalue_5 (`GameplayStatics.GetActorOfClass` _asbp_spawn_point_4))
            (`self.K2_TeleportTo` :`self` _returnvalue :`DestLocation` (`self.K2_GetActorLocation` _returnvalue_5)) ; Spawn Point 3
          ))))
    (set `self.Actor3Active` true)))

(event `SpawnActor1`
  ;[1 1 1] Spawn Actor 1
  (`KismetSystemLibrary.Delay` 0.0) ; Prevents Spawning At Same Points
  (if (not (`self.Actor1Active`))
    (bind _asbp_cube (castclass `/Game/RandomPointSpawner/Actors/BP_Cube` "/Game/RandomPointSpawner/Actors/BP_Cube.BP_Cube_C")) ; Cast To Actor 1
    (bind _returnvalue (`GameplayStatics.GetActorOfClass` _asbp_cube))
    (`|MultiGate` true :!label _label_2 ; Spawn At Random Point
      (:`Out 0`
        (if (`self.SpawnPoint1Active`)
          (goto _label_2)
          (else
            (set `self.SpawnPoint1Active` true) ; Set Spawn Point As Active (Used)
            (bind _asbp_spawn_point_1 (castclass `/Game/RandomPointSpawner/SpawnPoints/BP_SpawnPoint1` "/Game/RandomPointSpawner/SpawnPoints/BP_SpawnPoint1.BP_SpawnPoint1_C"))
            (bind _returnvalue_2 (`GameplayStatics.GetActorOfClass` _asbp_spawn_point_1))
            (`self.K2_TeleportTo` :`self` _returnvalue :`DestLocation` (`self.K2_GetActorLocation` _returnvalue_2)) ; Spawn Point 1
          )))
      (:`Out 1`
        (if (`self.SpawnPoint2Active`)
          (goto _label_2)
          (else
            (set `self.SpawnPoint2Active` true)
            (bind _asbp_spawn_point_2 (castclass `/Game/RandomPointSpawner/SpawnPoints/BP_SpawnPoint2` "/Game/RandomPointSpawner/SpawnPoints/BP_SpawnPoint2.BP_SpawnPoint2_C"))
            (bind _returnvalue_3 (`GameplayStatics.GetActorOfClass` _asbp_spawn_point_2))
            (`self.K2_TeleportTo` :`self` _returnvalue :`DestLocation` (`self.K2_GetActorLocation` _returnvalue_3)) ; Spawn Point 2
          )))
      (:`Out 2`
        (if (`self.SpawnPoint3Active`)
          (goto _label_2)
          (else
            (set `self.SpawnPoint3Active` true)
            (bind _asbp_spawn_point_3 (castclass `/Game/RandomPointSpawner/SpawnPoints/BP_SpawnPoint3` "/Game/RandomPointSpawner/SpawnPoints/BP_SpawnPoint3.BP_SpawnPoint3_C"))
            (bind _returnvalue_4 (`GameplayStatics.GetActorOfClass` _asbp_spawn_point_3))
            (`self.K2_TeleportTo` :`self` _returnvalue :`DestLocation` (`self.K2_GetActorLocation` _returnvalue_4)) ; Spawn Point 3
          )))
      (:`Out 3`
        (if (`self.SpawnPoint4Active`)
          (goto _label_2)
          (else
            (set `self.SpawnPoint4Active` true)
            (bind _asbp_spawn_point_4 (castclass `/Game/RandomPointSpawner/SpawnPoints/BP_SpawnPoint4` "/Game/RandomPointSpawner/SpawnPoints/BP_SpawnPoint4.BP_SpawnPoint4_C"))
            (bind _returnvalue_5 (`GameplayStatics.GetActorOfClass` _asbp_spawn_point_4))
            (`self.K2_TeleportTo` :`self` _returnvalue :`DestLocation` (`self.K2_GetActorLocation` _returnvalue_5)) ; Spawn Point 4
          ))))
    (set `self.Actor1Active` true) ; Set Actor As Spawned
  ))

(event `SpawnActor2`
  ;[1 1 1] Spawn Actor 2
  (`KismetSystemLibrary.Delay` 0.4)
  (if (not (`self.Actor2Active`))
    (bind _asbp_cylinder (castclass `/Game/RandomPointSpawner/Actors/BP_Cylinder` "/Game/RandomPointSpawner/Actors/BP_Cylinder.BP_Cylinder_C"))
    (bind _returnvalue (`GameplayStatics.GetActorOfClass` _asbp_cylinder))
    (`|MultiGate` true :!label _label_3 ; Spawn At Random Point
      (:`Out 0`
        (if (`self.SpawnPoint1Active`)
          (goto _label_3)
          (else
            (set `self.SpawnPoint1Active` true) ; Set Spawn Point As Active (Used)
            (bind _asbp_spawn_point_1 (castclass `/Game/RandomPointSpawner/SpawnPoints/BP_SpawnPoint1` "/Game/RandomPointSpawner/SpawnPoints/BP_SpawnPoint1.BP_SpawnPoint1_C"))
            (bind _returnvalue_2 (`GameplayStatics.GetActorOfClass` _asbp_spawn_point_1))
            (`self.K2_TeleportTo` :`self` _returnvalue :`DestLocation` (`self.K2_GetActorLocation` _returnvalue_2)) ; Spawn Point 1
          )))
      (:`Out 1`
        (if (`self.SpawnPoint2Active`)
          (goto _label_3)
          (else
            (set `self.SpawnPoint2Active` true)
            (bind _asbp_spawn_point_2 (castclass `/Game/RandomPointSpawner/SpawnPoints/BP_SpawnPoint2` "/Game/RandomPointSpawner/SpawnPoints/BP_SpawnPoint2.BP_SpawnPoint2_C"))
            (bind _returnvalue_3 (`GameplayStatics.GetActorOfClass` _asbp_spawn_point_2))
            (`self.K2_TeleportTo` :`self` _returnvalue :`DestLocation` (`self.K2_GetActorLocation` _returnvalue_3)) ; Spawn Point 2
          )))
      (:`Out 2`
        (if (`self.SpawnPoint3Active`)
          (goto _label_3)
          (else
            (set `self.SpawnPoint3Active` true)
            (bind _asbp_spawn_point_3 (castclass `/Game/RandomPointSpawner/SpawnPoints/BP_SpawnPoint3` "/Game/RandomPointSpawner/SpawnPoints/BP_SpawnPoint3.BP_SpawnPoint3_C"))
            (bind _returnvalue_4 (`GameplayStatics.GetActorOfClass` _asbp_spawn_point_3))
            (`self.K2_TeleportTo` :`self` _returnvalue :`DestLocation` (`self.K2_GetActorLocation` _returnvalue_4)) ; Spawn Point 3
          )))
      (:`Out 3`
        (if (`self.SpawnPoint4Active`)
          (goto _label_3)
          (else
            (set `self.SpawnPoint4Active` true)
            (bind _asbp_spawn_point_4 (castclass `/Game/RandomPointSpawner/SpawnPoints/BP_SpawnPoint4` "/Game/RandomPointSpawner/SpawnPoints/BP_SpawnPoint4.BP_SpawnPoint4_C"))
            (bind _returnvalue_5 (`GameplayStatics.GetActorOfClass` _asbp_spawn_point_4))
            (`self.K2_TeleportTo` :`self` _returnvalue :`DestLocation` (`self.K2_GetActorLocation` _returnvalue_5)) ; Spawn Point 3
          ))))
    (set `self.Actor2Active` true)))

(event `SpawnActor4`
  ;[1 1 1] Spawn Actor 4
  (`KismetSystemLibrary.Delay` 1.0)
  (if (not (`self.Actor4Active`))
    (bind _asbp_cone (castclass `/Game/RandomPointSpawner/Actors/BP_Cone` "/Game/RandomPointSpawner/Actors/BP_Cone.BP_Cone_C"))
    (bind _returnvalue (`GameplayStatics.GetActorOfClass` _asbp_cone))
    (`|MultiGate` true :!label _label_4 ; Spawn At Random Point
      (:`Out 0`
        (if (`self.SpawnPoint1Active`)
          (goto _label_4)
          (else
            (set `self.SpawnPoint1Active` true) ; Set Spawn Point As Active (Used)
            (bind _asbp_spawn_point_1 (castclass `/Game/RandomPointSpawner/SpawnPoints/BP_SpawnPoint1` "/Game/RandomPointSpawner/SpawnPoints/BP_SpawnPoint1.BP_SpawnPoint1_C"))
            (bind _returnvalue_2 (`GameplayStatics.GetActorOfClass` _asbp_spawn_point_1))
            (`self.K2_TeleportTo` :`self` _returnvalue :`DestLocation` (`self.K2_GetActorLocation` _returnvalue_2)) ; Spawn Point 1
          )))
      (:`Out 1`
        (if (`self.SpawnPoint2Active`)
          (goto _label_4)
          (else
            (set `self.SpawnPoint2Active` true)
            (bind _asbp_spawn_point_2 (castclass `/Game/RandomPointSpawner/SpawnPoints/BP_SpawnPoint2` "/Game/RandomPointSpawner/SpawnPoints/BP_SpawnPoint2.BP_SpawnPoint2_C"))
            (bind _returnvalue_3 (`GameplayStatics.GetActorOfClass` _asbp_spawn_point_2))
            (`self.K2_TeleportTo` :`self` _returnvalue :`DestLocation` (`self.K2_GetActorLocation` _returnvalue_3)) ; Spawn Point 2
          )))
      (:`Out 2`
        (if (`self.SpawnPoint3Active`)
          (goto _label_4)
          (else
            (set `self.SpawnPoint3Active` true)
            (bind _asbp_spawn_point_3 (castclass `/Game/RandomPointSpawner/SpawnPoints/BP_SpawnPoint3` "/Game/RandomPointSpawner/SpawnPoints/BP_SpawnPoint3.BP_SpawnPoint3_C"))
            (bind _returnvalue_4 (`GameplayStatics.GetActorOfClass` _asbp_spawn_point_3))
            (`self.K2_TeleportTo` :`self` _returnvalue :`DestLocation` (`self.K2_GetActorLocation` _returnvalue_4)) ; Spawn Point 3
          )))
      (:`Out 3`
        (if (`self.SpawnPoint4Active`)
          (goto _label_4)
          (else
            (set `self.SpawnPoint4Active` true)
            (bind _asbp_spawn_point_4 (castclass `/Game/RandomPointSpawner/SpawnPoints/BP_SpawnPoint4` "/Game/RandomPointSpawner/SpawnPoints/BP_SpawnPoint4.BP_SpawnPoint4_C"))
            (bind _returnvalue_5 (`GameplayStatics.GetActorOfClass` _asbp_spawn_point_4))
            (`self.K2_TeleportTo` :`self` _returnvalue :`DestLocation` (`self.K2_GetActorLocation` _returnvalue_5)) ; Spawn Point 3
          ))))
    (set `self.Actor4Active` true)))

(fn `UserConstructionScript`)