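; Extinguishable fire actor with looping-style flame effects, an attenuated fire sound and a health value.
; Its Box_F trigger sets an overlap flag on any Fire_Ex actor entering or leaving it.
; Tick polls FireHealth, shutting off Niagara effects in stages as it drops.
; At zero it removes fire components, activates dissolving smoke, fades the sound through a timeline, then destroys itself.
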(event `self.ReceiveBeginPlay`
  (bind _returnvalue (`GameplayStatics.SpawnSoundAtLocation` "/Game/StarterContent/Audio/Fire01_Cue.Fire01_Cue" (`self.K2_GetActorLocation`) (struct) 1.0 1.0 0.0 "/Game/Sound/NewSoundAttenuation.NewSoundAttenuation" null))
  (set `self.FireSound` _returnvalue))

(event `self.ReceiveTick`
  (params (DeltaSeconds :type "Float (single-precision)"))
  (bind _firehealth (`self.FireHealth`))
  (bind _firesound (`self.FireSound`))
  (`|ExecutionSequence`
    (:`then_0`
      (if (<= _firehealth 70.0)
        (`ActorComponent.Deactivate` (`self.Niagara2`))))
    (:`then_1`
      (if (<= _firehealth 40.0)
        (`ActorComponent.Deactivate` (`self.Niagara1`))))
    (:`then_2`
      (if (<= (`self.FireHealth`) 0.0)
        (`ActorComponent.K2_DestroyComponent` (`self.w_fire`))
        (`ActorComponent.K2_DestroyComponent` (`self.Box_F`))
        (`ActorComponent.Activate` (`self.NS_SmokeDissolve1a`) false)
        (`ActorComponent.Deactivate` (`self.Niagara1`))
        (`ActorComponent.Deactivate` (`self.Niagara2`))
        (`ActorComponent.Deactivate` (`self.Niagara`))
        (bind (_direction _newtrack_0) (`Timeline|SoundVolumeTimeline`)
          (:`Update`
            (`AudioComponent.SetVolumeMultiplier` _firesound _newtrack_0))
          (:`Finished`
            (`self.K2_DestroyActor`)
            (`AudioComponent.Stop` _firesound)
            (`ActorComponent.K2_DestroyComponent` _firesound)))))))

(event `self.Box_F.OnComponentBeginOverlap`
  (params (OverlappedComponent :type "PrimitiveComponent Object Reference") (OtherActor :type "Actor Object Reference") (OtherComp :type "PrimitiveComponent Object Reference") (OtherBodyIndex :type Integer) (bFromSweep :type Boolean) (SweepResult :type "HitResult Structure (by ref)"))
  (bind _asfire_ex (cast `/Game/VRTemplate/Blueprints/Fire_Ex` OtherActor))
  (set `/Game/VRTemplate/Blueprints/Fire_Ex.Overlap_F` true _asfire_ex))

(event `self.Box_F.OnComponentEndOverlap`
  (params (OverlappedComponent :type "PrimitiveComponent Object Reference") (OtherActor :type "Actor Object Reference") (OtherComp :type "PrimitiveComponent Object Reference") (OtherBodyIndex :type Integer))
  (bind _asfire_ex (cast `/Game/VRTemplate/Blueprints/Fire_Ex` OtherActor))
  (set `/Game/VRTemplate/Blueprints/Fire_Ex.Overlap_F` false _asfire_ex))

(fn `UserConstructionScript`)