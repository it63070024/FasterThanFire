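; Noti_3 is a one-shot trigger that halts the VR player and moves a Fire_ex_noti notification actor to the player.
; The first overlap with its Box, unfiltered by actor, sets the VRPawn's MaxWalkSpeed to zero.
; It then moves the Fire_ex_noti actor to the pawn's VRCharacterOrigin location, finding both actors by class lookup.
; An unconnected branch would enable custom depth rendering on the Activate_water mesh.
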(event `self.Box.OnComponentBeginOverlap`
  (params (OverlappedComponent :type "PrimitiveComponent Object Reference") (OtherActor :type "Actor Object Reference") (OtherComp :type "PrimitiveComponent Object Reference") (OtherBodyIndex :type Integer) (bFromSweep :type Boolean) (SweepResult :type "HitResult Structure (by ref)"))
  (`/Engine/EditorBlueprintResources/StandardMacros.DoOnce` false
    (:`Completed`
      (bind _outactors (`GameplayStatics.GetAllActorsOfClass` "/Game/VRTemplate/Blueprints/VRPawn.VRPawn_C"))
      (bind _output (`|GetArrayItem` _outactors))
      (set `CharacterMovementComponent.MaxWalkSpeed` 0.0 (`Character.CharacterMovement` _output))
      (bind _outactors_2 (`GameplayStatics.GetAllActorsOfClass` "/Game/Blueprint/Fire_ex_noti.Fire_ex_noti_C"))
      (`self.K2_SetActorLocation` (`|GetArrayItem` _outactors_2) (`SceneComponent.K2_GetComponentLocation` (`/Game/VRTemplate/Blueprints/VRPawn.VRCharacterOrigin` _output)) false false))))

(fn `UserConstructionScript`)