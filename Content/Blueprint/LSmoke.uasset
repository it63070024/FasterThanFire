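; LSmoke is a trigger actor that prompts the VR player with a notification until its widget is opened.
; Overlapping its box enables input and starts a looping timer that repeatedly calls the VRPawn's NotiL notification.
; Pressing IA_OpenNoti during overlap restores the widget's full white tint, stops the timer and notification light, and blocks future prompts.
; Leaving the box clears the timer, light and input.
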(event `EnhancedInput|/Game/VRTemplate/Input/Actions/IA_OpenNoti`
  (params (ActionValue :type Boolean) (ElapsedSeconds :type "Float (double-precision)") (TriggeredSeconds :type "Float (double-precision)") (InputAction :type "InputAction Object Reference" :default "/Game/VRTemplate/Input/Actions/IA_OpenNoti.IA_OpenNoti"))
  (:`Started`
    (if (`self.Can press`)
      (`KismetSystemLibrary.PrintString` "press")
      (`WidgetComponent.SetTintColorAndOpacity` (`self.Widget`) (make `LinearColor` 1.0 1.0 1.0 1.0))
      (set `self.AlreadyPress` true)
      (`KismetSystemLibrary.K2_ClearAndInvalidateTimerHandle` (stale `self.Box.OnComponentBeginOverlap` _returnvalue))
      (bind _asvrpawn (cast `/Game/VRTemplate/Blueprints/VRPawn` (`GameplayStatics.GetPlayerCharacter` 0)))
      (`LightComponent.SetIntensity` (`/Game/VRTemplate/Blueprints/VRPawn.NotiLight` _asvrpawn) 0.0)
      (`self.DisableInput` (`GameplayStatics.GetPlayerController` 0)))))

(event `self.Box.OnComponentBeginOverlap`
  (params (OverlappedComponent :type "PrimitiveComponent Object Reference") (OtherActor :type "Actor Object Reference") (OtherComp :type "PrimitiveComponent Object Reference") (OtherBodyIndex :type Integer) (bFromSweep :type Boolean) (SweepResult :type "HitResult Structure (by ref)"))
  (if (not (`self.AlreadyPress`))
    (bind _returnvalue (`KismetSystemLibrary.K2_SetTimerDelegate` (delegate `Noti`) 0.5 true))
    (set `self.Can press` true)
    (`self.EnableInput` (`GameplayStatics.GetPlayerController` 0))))

(event `Noti`
  (bind _asvrpawn (cast `/Game/VRTemplate/Blueprints/VRPawn` (`GameplayStatics.GetPlayerCharacter` 0)))
  (`/Game/VRTemplate/Blueprints/VRPawn.NotiL` _asvrpawn))

(event `self.Box.OnComponentEndOverlap`
  (params (OverlappedComponent :type "PrimitiveComponent Object Reference") (OtherActor :type "Actor Object Reference") (OtherComp :type "PrimitiveComponent Object Reference") (OtherBodyIndex :type Integer))
  (`KismetSystemLibrary.K2_ClearAndInvalidateTimerHandle` (stale `self.Box.OnComponentBeginOverlap` _returnvalue))
  (set `self.Can press` false)
  (bind _asvrpawn (cast `/Game/VRTemplate/Blueprints/VRPawn` (`GameplayStatics.GetPlayerCharacter` 0)))
  (`LightComponent.SetIntensity` (`/Game/VRTemplate/Blueprints/VRPawn.NotiLight` _asvrpawn) 0.0)
  (`self.DisableInput` (`GameplayStatics.GetPlayerController` 0)))

(fn `UserConstructionScript`)