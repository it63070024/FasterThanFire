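; One-shot notification trigger that freezes the VR player and shows a notification when its Box is overlapped.
; The first overlap casts player character 0 to VRPawn, sets its notification flags and zeroes its walk speed.
; It then retints the pawn's widgets, making Noti2 opaque while turning Timer and HUDWidget transparent.
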(event `self.Box.OnComponentBeginOverlap`
  (params (OverlappedComponent :type "PrimitiveComponent Object Reference") (OtherActor :type "Actor Object Reference") (OtherComp :type "PrimitiveComponent Object Reference") (OtherBodyIndex :type Integer) (bFromSweep :type Boolean) (SweepResult :type "HitResult Structure (by ref)"))
  (`/Engine/EditorBlueprintResources/StandardMacros.DoOnce` false
    (:`Completed`
      (bind _asvrpawn (cast `/Game/VRTemplate/Blueprints/VRPawn` (`GameplayStatics.GetPlayerCharacter` 0)))
      (set `/Game/VRTemplate/Blueprints/VRPawn.CloseNoti?` false _asvrpawn)
      (set `/Game/VRTemplate/Blueprints/VRPawn.shownotiblock` true _asvrpawn)
      (set `CharacterMovementComponent.MaxWalkSpeed` 0.0 (`Character.CharacterMovement` _asvrpawn))
      (`WidgetComponent.SetTintColorAndOpacity` (`/Game/VRTemplate/Blueprints/VRPawn.Timer` _asvrpawn) (make `LinearColor` 1.0 1.0 1.0))
      (`WidgetComponent.SetTintColorAndOpacity` (`/Game/VRTemplate/Blueprints/VRPawn.HUDWidget` _asvrpawn) (make `LinearColor` 1.0 1.0 1.0))
      (`WidgetComponent.SetTintColorAndOpacity` (`/Game/VRTemplate/Blueprints/VRPawn.Noti2` _asvrpawn) (make `LinearColor` 1.0 1.0 1.0 1.0)))))

(fn `UserConstructionScript`)