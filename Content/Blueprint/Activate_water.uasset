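; Trigger actor that sets off a fire alarm and sprinkler sequence to put out a fire when its box is overlapped.
; The overlap clears the mesh's custom depth, plays the alarm, and activates the first Water actor found in the level with sprinkler audio.
; After a delay it stops the first Fire_niagara actor's effect and sound, plays an extinguished cue, then fades out and deactivates the water.
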(event `self.Box.OnComponentBeginOverlap`
  (params (OverlappedComponent :type "PrimitiveComponent Object Reference") (OtherActor :type "Actor Object Reference") (OtherComp :type "PrimitiveComponent Object Reference") (OtherBodyIndex :type Integer) (bFromSweep :type Boolean) (SweepResult :type "HitResult Structure (by ref)"))
  (bind _watersound (`self.WaterSound`))
  (`GameplayStatics.PlaySound2D` "/Game/Sound/SoundCue/FireAlarmCue.FireAlarmCue" 0.7 1.0 0.0 null null)
  (`PrimitiveComponent.SetRenderCustomDepth` (`self.StaticMesh`) false)
  (bind _outactors (`GameplayStatics.GetAllActorsOfClass` "/Game/Blueprint/Water.Water_C"))
  (bind _output (`|GetArrayItem` _outactors))
  (bind _water (`/Game/Blueprint/Water.Water` _output))
  (`ActorComponent.Activate` _water false)
  (bind _returnvalue (`GameplayStatics.SpawnSoundAtLocation` "/Game/Sound/SoundCue/SprinklerCue.SprinklerCue" (`self.K2_GetActorLocation` _output) (struct) 0.74 1.0 0.0 null null))
  (set `self.WaterSound` _returnvalue)
  (`KismetSystemLibrary.Delay` 5.0)
  (bind _outactors_2 (`GameplayStatics.GetAllActorsOfClass` "/Game/Blueprint/Fire_niagara.Fire_niagara_C"))
  (bind _output_2 (`|GetArrayItem` _outactors_2))
  (`AudioComponent.Stop` (`/Game/Blueprint/Fire_niagara.FireSFX` _output_2))
  (`ActorComponent.Deactivate` (`/Game/Blueprint/Fire_niagara.Niagara` _output_2))
  (`GameplayStatics.PlaySoundAtLocation` "/Game/Sound/SoundCue/FireExtinguishedCue.FireExtinguishedCue" (`self.K2_GetActorLocation` _output_2) (struct) 1.0 1.0 0.0 null null null null)
  (`AudioComponent.FadeOut` _watersound 3.0 0.0 "Linear")
  (`KismetSystemLibrary.Delay` 3.0)
  (`AudioComponent.Stop` _watersound)
  (`ActorComponent.Deactivate` _water))

(fn `UserConstructionScript`)