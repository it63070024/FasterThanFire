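; Smartwatch actor attached to the player character, with a paged widget UI, beeps, a notification queue and a navigation waypoint.
; After a short delay it initializes if the parent character has an AC_SmartWatch component, filling the main UI's switcher from SmartWatchPages.
; Notifications show one by one while the watch is active, blocking page switching, and dispatchers report state changes.
; The construction script applies the case material from a data table row.
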(event `self.ReceiveBeginPlay`
  (bind _returnvalue (`self.GetAttachParentActor`))
  ;[0.7957 1 0.1686] Check if smartwatch is already attached on character
  (if (`KismetMathLibrary.ClassIsChildOf` (`GameplayStatics.GetObjectClass` _returnvalue) "/Script/Engine.Character")
    (bind _ascharacter (cast `Character` _returnvalue))
    (set `self.ParentCharacter` _ascharacter))
  ;[0.7294 1 0.2191] Initialize watch and check if there are valid references
  (`KismetSystemLibrary.Delay` 0.32)
  (`self.InitializeWatch`))

(event `InitializeWatch`
  (bind _as_wbp_smart_watch_main (`self.As WBP Smart Watch Main`))
  (if (not (`self.IsInitialized`))
    ;[1 1 1] Check valid objects
    (if (`KismetSystemLibrary.IsValid` (`self.ParentCharacter`))
      (if (`KismetSystemLibrary.IsValid` (`self.GetComponentByClass` (`self.ParentCharacter`) "/Game/SmartWatch/Assets/Blueprints/AC_SmartWatch.AC_SmartWatch_C"))
        (set `self.IsInitialized` true)
        ;[0 0.8267 1] Get main ui widget
        (bind _returnvalue (`|CreateWidget` "/Game/SmartWatch/Assets/Widgets/WBP_SmartWatch_MainUI.WBP_SmartWatch_MainUI_C" null (`self.ParentCharacter`)))
        (`WidgetComponent.SetWidget` (`self.DeviceWidget`) _returnvalue)
        (set `self.As WBP Smart Watch Main` _returnvalue)
        ;[0 0.3175 1] Add pages to the main ui
        (for _array_element (`self.SmartWatchPages`)
          (bind _returnvalue_2 (`|CreateWidget` _array_element (`GameplayStatics.GetPlayerController` 0)))
          (if (`KismetSystemLibrary.IsValid` _as_wbp_smart_watch_main)
            (`PanelWidget.AddChild` (`/Game/SmartWatch/Assets/Widgets/WBP_SmartWatch_MainUI.UI_Switch` _as_wbp_smart_watch_main) _returnvalue_2)))
        (else
          (`KismetSystemLibrary.PrintString` "\"BP_SmartWatch_Device\" has not found a \"AC_SmartWatch\" component in your character bp. \n \nPlease add \"AC_SmartWatch\" component to your player character!" true true (struct :`R` 1.0 :`G` 0.035166 :`A` 1.0) 60.0)))
      (else
        (`KismetSystemLibrary.PrintString` "The \"BP_SmartWatch_Device\" class has not found a valid character parent. \n \nPlease add a \"AC_SmartWatch\" component to the same character bp the \"BP_SmartWatch_Device\" is attached to!" true true (struct :`R` 1.0 :`G` 0.035166 :`A` 1.0) 20.0)))))

(event `self.ActivateWatch`
  (if (`self.IsInitialized`)
    (set `self.IsActivated` true)
    ;[0.5686 0.4784 1] optional beep sound when watch is showing up
    (if (`self.BeepSoundOnActivating`)
      (`KismetSystemLibrary.Delay` 0.5)
      (if (not (`self.IsPlayingBeepSound`))
        (`self.PlayBeepSound` 2 0.2 0.13)))
    ;[1 0 0.2902] Check if there are notifications in queue
    (if (> (`KismetMathLibrary.Conv_IntToDouble` (`KismetArrayLibrary.Array_Length` (`self.StoredNotifications`))) 0.0)
      (`self.DequeueNotifications`))
    ;[0.4549 1 0.02924] Call activate dispatcher
    (`self.WachtedActivateStateChanged` true)))

(event `self.DeactivateWatch`
  (if (`self.IsInitialized`)
    (set `self.IsActivated` false)
    ;[0.4549 1 0.02924] Call deactivate dispatcher
    (`self.WachtedActivateStateChanged` false)))

(event `self.SwitchUI`
  (params (SwitchMode :type "/Game/SmartWatch/Assets/Data/DataTypes/E_SmartWatch_SwitchMode Enum" :default "NewEnumerator0"))
  (bind _as_wbp_smart_watch_main (`self.As WBP Smart Watch Main`))
  (if (`self.IsInitialized`)
    (if (not (`self.IsShowingNotification`))
      ;[1 0.9765 0.3804] Switch page on smartwatch UI
      (`/Game/SmartWatch/Assets/Widgets/WBP_SmartWatch_MainUI.SwitchUI` (`self.As WBP Smart Watch Main`) SwitchMode)
      (`self.SmartWatchPageChanged` (`/Game/SmartWatch/Assets/Widgets/WBP_SmartWatch_MainUI.CurrentPageIndex` _as_wbp_smart_watch_main) (`WidgetSwitcher.GetActiveWidget` (`/Game/SmartWatch/Assets/Widgets/WBP_SmartWatch_MainUI.UI_Switch` _as_wbp_smart_watch_main))))))

(event `self.SwitchToPage`
  (params (Page :type "UserWidget Class Reference"))
  (bind _as_wbp_smart_watch_main (`self.As WBP Smart Watch Main`))
  (if (`self.IsInitialized`)
    (if (not (`self.IsShowingNotification`))
      ;[1 0.9765 0.3804] Switch to a specific page on smartwatch UI
      (`/Game/SmartWatch/Assets/Widgets/WBP_SmartWatch_MainUI.SwitchToPage` (`self.As WBP Smart Watch Main`) Page)
      (`self.SmartWatchPageChanged` (`/Game/SmartWatch/Assets/Widgets/WBP_SmartWatch_MainUI.CurrentPageIndex` _as_wbp_smart_watch_main) (`WidgetSwitcher.GetActiveWidget` (`/Game/SmartWatch/Assets/Widgets/WBP_SmartWatch_MainUI.UI_Switch` _as_wbp_smart_watch_main))))))

(event `self.PlayBeepSound`
  (params (BeepCount :type Integer) (BeepDelay :type "Float (double-precision)") (Volume :type "Float (double-precision)") (Pitch :type "Float (double-precision)"))
  (if (`self.IsInitialized`)
    ;[0.5686 0.4784 1] Plays a amount of beeps with a specific delay and volume / pitch
    (set `self.IsPlayingBeepSound` true)
    (`/Game/SmartWatch/Assets/Blueprints/BP_SmartWatch_LoopWithDelay.ForLoopWithDelay` BeepCount BeepDelay
      (:`then_0`
        (`GameplayStatics.PlaySoundAtLocation` "/Game/SmartWatch/Assets/Sounds/S_SmartWatch_Beep.S_SmartWatch_Beep" (`self.K2_GetActorLocation`) (struct) Volume Pitch 0.0 null null null null))
      (:`Completed`
        (set `self.IsPlayingBeepSound` false)))))

(event `self.AddNotification`
  (params (NotificationInfo :type "/Game/SmartWatch/Assets/Data/DataTypes/F_SmartWatch_NotificationInfo Structure"))
  ;[1 0 0.8431] Notifications
  (if (`self.IsInitialized`)
    ;;[0.5686 0.4784 1] Play notification sound
    (if (and (`.WithBeepSound_8_813D391E4746909746071188D880EEED` (break `/Game/SmartWatch/Assets/Data/DataTypes/F_SmartWatch_NotificationInfo` NotificationInfo)) (not (`self.IsPlayingBeepSound`)))
      (`self.PlayBeepSound` 6 0.2 0.15 0.82))
    (`KismetArrayLibrary.Array_Add` (`self.StoredNotifications`) NotificationInfo)
    (`/Game/SmartWatch/Assets/Widgets/WBP_SmartWatch_MainUI.UpdateNotificationScreens` (`self.As WBP Smart Watch Main`))
    (`self.NotificationAdded`)))

(event `DequeueNotifications`
  (bind _output (`|GetArrayItem` (`self.StoredNotifications`)))
  ;[1 0 0.8431] Notifications
  ;;[1 0 0.2902] Dequeue notifications
  (if (`self.IsInitialized`)
    (if (not (`self.IsShowingNotification`))
      (set `self.IsShowingNotification` true)
      (`/Game/SmartWatch/Assets/Widgets/WBP_SmartWatch_MainUI.ShowNotification` (`self.As WBP Smart Watch Main`) _output)
      (`KismetSystemLibrary.Delay` (`.Duration_6_EFBF7037448FEAF14B2DFBAEA617F11C` (break `/Game/SmartWatch/Assets/Data/DataTypes/F_SmartWatch_NotificationInfo` _output)))
      (`KismetArrayLibrary.Array_Remove` (`self.StoredNotifications`))
      (`self.NotificationFinished`)
      (if (> (`KismetArrayLibrary.Array_Length` (`self.StoredNotifications`)) 0)
        (set `self.IsShowingNotification` false)
        (if (`self.IsActivated`)
          (`self.DequeueNotifications`))
        (else
          (set `self.IsShowingNotification` false))))))

(event `self.ClearNotificationQueue`
  ;[1 0 0.8431] Notifications
  ;;[1 0 0.2902] Clear all upcoming notifications
  (if (`self.IsInitialized`)
    (`KismetArrayLibrary.Array_Clear` (`self.StoredNotifications`))
    (`/Game/SmartWatch/Assets/Widgets/WBP_SmartWatch_MainUI.UpdateNotificationScreens` (`self.As WBP Smart Watch Main`))))

(event `self.SetNewNavigationWaypoint`
  (params (WaypointInfo :type "/Game/SmartWatch/Assets/Data/DataTypes/F_SmartWatch_WaypointInfo Structure"))
  ;[0.9333 1 0] Navigation waypoint
  (if (`self.IsInitialized`)
    (set `self.CurrentNavigationWaypoint` WaypointInfo)))

(event `self.ClearNavigationWaypoint`
  ;[0.9333 1 0] Navigation waypoint
  (if (`self.IsInitialized`)
    (set `self.CurrentNavigationWaypoint` (struct))))

(fn `UserConstructionScript`
  (bind (_datatable _rowname) (break `DataTableRowHandle` (`self.Case style`)))
  ;[0 0.5678 1] Set case style
  (bind _returnvalue (`|GetDataTableRow` _datatable _rowname)
    (:`then`
      (`PrimitiveComponent.SetMaterial` (`self.Mesh_SmartWatch`) 0 (`.Material_Instance_5_6E4FD85845A9DD0E288448A709E30171` (break `/Game/SmartWatch/Assets/Data/DataTypes/F_SmartWatch_Styles` _returnvalue))))))