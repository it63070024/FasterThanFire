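; Actor component that gives a Character a usable smart watch, forwarding commands to an attached BP_SmartWatch_Device actor.
; It looks up that device before each command, then shows or hides it with a montage and a toggle cooldown.
; It also relays page switching, notifications and navigation waypoints, raising state and page change calls.
; When the device enables it, notification events add or remove an on-screen hint widget.
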(event `self.ReceiveBeginPlay`
  ;[0 1 0.3469] Get character owner ref
  (bind _ascharacter (cast `Character` (`self.GetOwner`))
    (:`then`
      (set `self.PlayerCharacterOwner` _ascharacter)
      ;[0 0.8021 1] Get smart watch actor ref
      (bind _hasbeenfound (`self.SetSmartWatchObj`))
      (if _hasbeenfound
        (`/Game/SmartWatch/Assets/Blueprints/BP_SmartWatch_Device.InitializeWatch` (`self.SmartWatchObj`))))
    (:`CastFailed`
      (`KismetSystemLibrary.PrintString` "The \"AC_SmartWatch\" class was added to a none character class. \n \nPlease only attach the actor component to a valid character bp." true true (struct :`R` 1.0 :`G` 0.035166 :`A` 1.0) 60.0))))

(event `ShowSmartWatch`
  ;[1 1 1] Start using smartwatch with animation
  (bind _hasbeenfound (`self.SetSmartWatchObj`))
  (if _hasbeenfound
    (if (not (`self.IsUsingSmartWatch`))
      (set `self.IsUsingSmartWatch` true)
      (`/Game/SmartWatch/Assets/Blueprints/BP_SmartWatch_Device.ActivateWatch` (`self.SmartWatchObj`))
      ;;[1 0.82 0] Adjust to your own animation system
      (`Character.PlayAnimMontage` (`self.PlayerCharacterOwner`) (`self.SmartWatchAnimMontage`) 1.0 "None")
      (`self.SmartWatchUsedStateChanged` true))))

(event `InitializeNotificationScreenHint`
  ;[1 0 0.9339] Notification hint icon on UI
  (add `/Game/SmartWatch/Assets/Blueprints/BP_SmartWatch_Device.NotificationAdded` (`self.SmartWatchObj`) (delegate `NotificationAdded`))
  (add `/Game/SmartWatch/Assets/Blueprints/BP_SmartWatch_Device.NotificationFinished` (`self.SmartWatchObj`) (delegate `NotificationFinished`)))

(event `NotificationAdded`
  ;[1 0 0.9339] Notification hint icon on UI
  (`self.UpdateNotificationScreenHint`))

(event `NotificationFinished`
  ;[1 0 0.9339] Notification hint icon on UI
  (`self.UpdateNotificationScreenHint`))

(event `UpdateNotificationScreenHint`
  ;[1 0 0.9339] Notification hint icon on UI
  (if (> (`KismetArrayLibrary.Array_Length` (`/Game/SmartWatch/Assets/Blueprints/BP_SmartWatch_Device.StoredNotifications` (`self.SmartWatchObj`))) 0)
    (if (not (`KismetSystemLibrary.IsValid` (`self.NotificationHintWidget`)))
      (bind _returnvalue (`|CreateWidget` "/Game/SmartWatch/Assets/Widgets/WBP_SmartWatch_NotificationHint.WBP_SmartWatch_NotificationHint_C"))
      (`UserWidget.AddToViewport` _returnvalue 0)
      (set `self.NotificationHintWidget` _returnvalue))
    (elif (`KismetSystemLibrary.IsValid` (`self.NotificationHintWidget`))
      (`Widget.RemoveFromParent` (`self.NotificationHintWidget`))
      (set `self.NotificationHintWidget` null))))

(event `HideSmartWatch`
  ;[1 1 1] Stop using smartwatch with animation
  (bind _hasbeenfound (`self.SetSmartWatchObj`))
  (if _hasbeenfound
    (if (`self.IsUsingSmartWatch`)
      (set `self.IsUsingSmartWatch` false)
      ;;[1 0.82 0] Adjust to your own animation system
      (`Character.StopAnimMontage` (`self.PlayerCharacterOwner`) (`self.SmartWatchAnimMontage`))
      (`/Game/SmartWatch/Assets/Blueprints/BP_SmartWatch_Device.DeactivateWatch` (`self.SmartWatchObj`))
      (`self.SmartWatchUsedStateChanged` false))))

(event `ShowHideSmartWatch`
  ;[0.7552 1 0.3708] Toggle smartwatch show / hide
  (if (not (`self.IsSmartWatchCooldown`))
    (set `self.IsSmartWatchCooldown` true)
    (if (not (`self.IsUsingSmartWatch`))
      (`self.ShowSmartWatch`)
      (`KismetSystemLibrary.Delay` 0.5)
      (set `self.IsSmartWatchCooldown` false)
      (else
        (`self.HideSmartWatch`)
        (`KismetSystemLibrary.Delay` 0.5)
        (set `self.IsSmartWatchCooldown` false)))))

(event `/Game/SmartWatch/Assets/Blueprints/BPI_SmartWatch.SwitchUI`
  (params (SwitchMode :type "/Game/SmartWatch/Assets/Data/DataTypes/E_SmartWatch_SwitchMode Enum" :default "NewEnumerator0"))
  ;[0.7145 0.6972 1] Switch smartwatch ui to the next page
  (bind _hasbeenfound (`self.SetSmartWatchObj`))
  (if _hasbeenfound
    (if (`self.IsUsingSmartWatch`)
      (`/Game/SmartWatch/Assets/Blueprints/BPI_SmartWatch.SwitchUI` (`self.SmartWatchObj`) SwitchMode)
      (bind _aswbp_smart_watch_main_ui (cast `/Game/SmartWatch/Assets/Widgets/WBP_SmartWatch_MainUI` (`WidgetComponent.GetWidget` (`/Game/SmartWatch/Assets/Blueprints/BP_SmartWatch_Device.DeviceWidget` (`self.SmartWatchObj`)))))
      (`self.SmartWatchPageChanged` (`/Game/SmartWatch/Assets/Widgets/WBP_SmartWatch_MainUI.CurrentPageIndex` _aswbp_smart_watch_main_ui) (`WidgetSwitcher.GetActiveWidget` (`/Game/SmartWatch/Assets/Widgets/WBP_SmartWatch_MainUI.UI_Switch` _aswbp_smart_watch_main_ui))))))

(event `/Game/SmartWatch/Assets/Blueprints/BPI_SmartWatch.SwitchToPage`
  (params (Page :type "UserWidget Class Reference"))
  ;[0.4696 0.8276 1] Switch smartwatch to a specific ui page
  (bind _hasbeenfound (`self.SetSmartWatchObj`))
  (if _hasbeenfound
    (if (`self.IsUsingSmartWatch`)
      (`/Game/SmartWatch/Assets/Blueprints/BP_SmartWatch_Device.SwitchToPage` (`self.SmartWatchObj`) Page)
      (bind _aswbp_smart_watch_main_ui (cast `/Game/SmartWatch/Assets/Widgets/WBP_SmartWatch_MainUI` (`WidgetComponent.GetWidget` (`/Game/SmartWatch/Assets/Blueprints/BP_SmartWatch_Device.DeviceWidget` (`self.SmartWatchObj`)))))
      (`self.SmartWatchPageChanged` (`/Game/SmartWatch/Assets/Widgets/WBP_SmartWatch_MainUI.CurrentPageIndex` _aswbp_smart_watch_main_ui) (`WidgetSwitcher.GetActiveWidget` (`/Game/SmartWatch/Assets/Widgets/WBP_SmartWatch_MainUI.UI_Switch` _aswbp_smart_watch_main_ui))))))

(event `/Game/SmartWatch/Assets/Blueprints/BPI_SmartWatch.AddNotification`
  (params (NotificationInfo :type "/Game/SmartWatch/Assets/Data/DataTypes/F_SmartWatch_NotificationInfo Structure"))
  ;[1 0 0.7607] Add a new notification to the smartwatch notification queue
  (bind _hasbeenfound (`self.SetSmartWatchObj`))
  (if _hasbeenfound
    (if (`self.IsUsingSmartWatch`)
      (`/Game/SmartWatch/Assets/Blueprints/BPI_SmartWatch.AddNotification` (`self.SmartWatchObj`) NotificationInfo)
      (`/Game/SmartWatch/Assets/Blueprints/BP_SmartWatch_Device.DequeueNotifications` (`self.SmartWatchObj`))
      (else
        (`/Game/SmartWatch/Assets/Blueprints/BPI_SmartWatch.AddNotification` (`self.SmartWatchObj`) NotificationInfo)))))

(event `/Game/SmartWatch/Assets/Blueprints/BPI_SmartWatch.ClearNotificationQueue`
  ;[1 0 0.08259] Clear upcoming notification queue
  (bind _hasbeenfound (`self.SetSmartWatchObj`))
  (if _hasbeenfound
    (`/Game/SmartWatch/Assets/Blueprints/BP_SmartWatch_Device.ClearNotificationQueue` (`self.SmartWatchObj`))))

(event `/Game/SmartWatch/Assets/Blueprints/BPI_SmartWatch.SetNewNavigationWaypoint`
  (params (WaypointInfo :type "/Game/SmartWatch/Assets/Data/DataTypes/F_SmartWatch_WaypointInfo Structure"))
  ;[0.9333 1 0] Set / Clear navigation waypoint
  (bind _hasbeenfound (`self.SetSmartWatchObj`))
  (if _hasbeenfound
    (`/Game/SmartWatch/Assets/Blueprints/BPI_SmartWatch.SetNewNavigationWaypoint` (`self.SmartWatchObj`) WaypointInfo)))

(event `/Game/SmartWatch/Assets/Blueprints/BPI_SmartWatch.ClearNavigationWaypoint`
  ;[0.9333 1 0] Set / Clear navigation waypoint
  (bind _hasbeenfound (`self.SetSmartWatchObj`))
  (if _hasbeenfound
    (`/Game/SmartWatch/Assets/Blueprints/BPI_SmartWatch.ClearNavigationWaypoint` (`self.SmartWatchObj`))))

(fn `GetCurrentWayPoint`
  (returns (CurrentWaypoint :type "/Game/SmartWatch/Assets/Data/DataTypes/F_SmartWatch_WaypointInfo Structure"))
  (return (`/Game/SmartWatch/Assets/Blueprints/BP_SmartWatch_Device.CurrentNavigationWaypoint` (`self.SmartWatchObj`))))

(fn `GetCustomWorldTime`
  (returns (WorldTime :type "DateTime Structure"))
  (return (`KismetMathLibrary.Now`)))

(fn `HasCurrentNavigationWaypoint`
  (returns (Result :type Boolean))
  (return (!= (`.Coordinates_3_539239F44E9BFE093E953897F3A6D9C3` (break `/Game/SmartWatch/Assets/Data/DataTypes/F_SmartWatch_WaypointInfo` (`/Game/SmartWatch/Assets/Blueprints/BP_SmartWatch_Device.CurrentNavigationWaypoint` (`self.SmartWatchObj`)))) (0.0 0.0 0.0) :`ErrorTolerance` 0.0)))

(fn `SetSmartWatchObj`
  (returns (HasBeenFound :type Boolean))
  (locals (Found :type Boolean))
  (for _array_element (`Actor.GetAttachedActors` (`self.PlayerCharacterOwner`) true false)
    (if (== (`GameplayStatics.GetObjectClass` _array_element) "/Game/SmartWatch/Assets/Blueprints/BP_SmartWatch_Device.BP_SmartWatch_Device_C")
      (bind _asbp_smart_watch_device (cast `/Game/SmartWatch/Assets/Blueprints/BP_SmartWatch_Device` _array_element))
      (set `self.SmartWatchObj` _asbp_smart_watch_device)
      (set `/Game/SmartWatch/Assets/Blueprints/BP_SmartWatch_Device.ParentCharacter` (`self.PlayerCharacterOwner`) (`self.SmartWatchObj`))
      (if (`/Game/SmartWatch/Assets/Blueprints/BP_SmartWatch_Device.ShowNotificationHintOnScreen` (`self.SmartWatchObj`))
        (`self.InitializeNotificationScreenHint`))
      (set `local.Found` true)))
  (if (not (`local.Found`))
    (`KismetSystemLibrary.PrintString` "No attached \"BP_SmartWatch_Device\" found in character bp." true true (struct :`R` 1.0 :`G` 0.312097 :`A` 1.0))
    (set `self.SmartWatchObj` null))
  (return (`local.Found`)))