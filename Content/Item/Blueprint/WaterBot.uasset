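; WaterBot is a spinning pickup that grants the VRPawn heat resistance on box overlap, then destroys itself.
; On BeginPlay, a random MultiGate picks one of four spawn point classes, teleporting the item to that actor and marking it active.
; An already active point only resets the gate, without a retry or teleport.
; Tick rotates the item in yaw steps throttled by a short Delay.
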(event `self.ReceiveBeginPlay`
  (`|MultiGate` true :!label _label ; Random Spawn
    (:`Out 0`
      (bind _asbp_spawn_point_1 (castclass `/Game/RandomPointSpawner/SpawnPoints/BP_SpawnPoint1` "/Game/RandomPointSpawner/SpawnPoints/BP_SpawnPoint1.BP_SpawnPoint1_C"))
      (bind _returnvalue (`GameplayStatics.GetActorOfClass` _asbp_spawn_point_1))
      (if (`self.IsActive`)
        (goto _label :!via `Reset`)
        (else
          (`|ExecutionSequence`
            (:`then_0`
              (`self.K2_TeleportTo` (`self.K2_GetActorLocation` _returnvalue)))
            (:`then_1`
              (`/Game/RandomPointSpawner/SpawnPoints/BP_SpawnPoint1.SetActive` _returnvalue))))))
    (:`Out 1`
      (bind _asbp_spawn_point_2 (castclass `/Game/RandomPointSpawner/SpawnPoints/BP_SpawnPoint2` "/Game/RandomPointSpawner/SpawnPoints/BP_SpawnPoint2.BP_SpawnPoint2_C"))
      (bind _returnvalue_2 (`GameplayStatics.GetActorOfClass` _asbp_spawn_point_2))
      (if (`self.IsActive`)
        (goto _label :!via `Reset`)
        (else
          (`|ExecutionSequence`
            (:`then_0`
              (`self.K2_TeleportTo` (`self.K2_GetActorLocation` _returnvalue_2)))
            (:`then_1`
              (`/Game/RandomPointSpawner/SpawnPoints/BP_SpawnPoint2.SetActive` _returnvalue_2))))))
    (:`Out 2`
      (bind _asbp_spawn_point_3 (castclass `/Game/RandomPointSpawner/SpawnPoints/BP_SpawnPoint3` "/Game/RandomPointSpawner/SpawnPoints/BP_SpawnPoint3.BP_SpawnPoint3_C"))
      (bind _returnvalue_3 (`GameplayStatics.GetActorOfClass` _asbp_spawn_point_3))
      (if (`self.IsActive`)
        (goto _label :!via `Reset`)
        (else
          (`|ExecutionSequence`
            (:`then_0`
              (`self.K2_TeleportTo` (`self.K2_GetActorLocation` _returnvalue_3)))
            (:`then_1`
              (`/Game/RandomPointSpawner/SpawnPoints/BP_SpawnPoint3.SetActive` _returnvalue_3))))))
    (:`Out 3`
      (bind _asbp_spawn_point_4 (castclass `/Game/RandomPointSpawner/SpawnPoints/BP_SpawnPoint4` "/Game/RandomPointSpawner/SpawnPoints/BP_SpawnPoint4.BP_SpawnPoint4_C"))
      (bind _returnvalue_4 (`GameplayStatics.GetActorOfClass` _asbp_spawn_point_4))
      (if (`self.IsActive`)
        (goto _label :!via `Reset`)
        (else
          (`|ExecutionSequence`
            (:`then_0`
              (`self.K2_TeleportTo` (`self.K2_GetActorLocation` _returnvalue_4)))
            (:`then_1`
              (`/Game/RandomPointSpawner/SpawnPoints/BP_SpawnPoint4.SetActive` _returnvalue_4))))))))

(event `self.ReceiveTick`
  (params (DeltaSeconds :type "Float (single-precision)"))
  (`KismetSystemLibrary.Delay` 0.05)
  (`self.K2_AddActorWorldRotation` (struct :`Yaw` 5.0)))

(event `self.Box.OnComponentBeginOverlap`
  (params (OverlappedComponent :type "PrimitiveComponent Object Reference") (OtherActor :type "Actor Object Reference") (OtherComp :type "PrimitiveComponent Object Reference") (OtherBodyIndex :type Integer) (bFromSweep :type Boolean) (SweepResult :type "HitResult Structure (by ref)"))
  (bind _asvrpawn (cast `/Game/VRTemplate/Blueprints/VRPawn` OtherActor))
  (set `/Game/VRTemplate/Blueprints/VRPawn.HeatResis` true _asvrpawn)
  (`self.K2_DestroyActor`))

(fn `UserConstructionScript`)