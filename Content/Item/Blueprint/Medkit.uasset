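; Medkit pickup actor that heals the VR player and spins slowly in the world.
; Overlapping its box with a VRPawn adds health, clamped to the maximum, prints the new value and destroys the actor.
; Tick applies a small rotation after a short delay.
; An unconnected random-spawn chain, built on a random MultiGate that would teleport it to one of four spawn points, never runs.
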(event `self.ReceiveBeginPlay`)

(event `self.ReceiveTick`
  (params (DeltaSeconds :type "Float (single-precision)"))
  (`KismetSystemLibrary.Delay` 0.05)
  (`self.K2_AddActorWorldRotation` (struct :`Yaw` 2.0)))

(event `self.Box.OnComponentBeginOverlap`
  (params (OverlappedComponent :type "PrimitiveComponent Object Reference") (OtherActor :type "Actor Object Reference") (OtherComp :type "PrimitiveComponent Object Reference") (OtherBodyIndex :type Integer) (bFromSweep :type Boolean) (SweepResult :type "HitResult Structure (by ref)"))
  (bind _asvrpawn (cast `/Game/VRTemplate/Blueprints/VRPawn` OtherActor))
  (bind _output_get (set `/Game/VRTemplate/Blueprints/VRPawn.PlayerCurrentHealth` (`KismetMathLibrary.FClamp` (+ (`/Game/VRTemplate/Blueprints/VRPawn.PlayerCurrentHealth` _asvrpawn) 25.0) 0.0 100.0) _asvrpawn))
  (`KismetSystemLibrary.PrintString` (`KismetStringLibrary.Conv_DoubleToString` _output_get))
  (`self.K2_DestroyActor`))

(fn `UserConstructionScript`)