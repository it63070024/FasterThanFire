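; BP_Cube is an actor with unfinished logic for teleporting itself to unoccupied spawn points, but BeginPlay is empty and none of that logic runs.
; The main disconnected chain teleports to BP_SpawnPoint3 and calls its SetActive, or, if active, uses a random MultiGate to try points 1 or 2.
; A separate orphaned chain handles BP_SpawnPoint4 likewise.
; Active points 1, 2 or 4 lead to a MultiGate reset.
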(event `self.ReceiveBeginPlay`)

(fn `UserConstructionScript`)