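; BP_Cylinder is an actor with draft logic for teleporting itself to a spawn point, currently inert because BeginPlay is empty and no event reaches the chains.
; Each branch finds a BP_SpawnPoint actor by class, checks IsActive, then either teleports there and calls SetActive or resets a MultiGate.
; An active SpawnPoint3 leads to a random MultiGate choosing between SpawnPoint1 and SpawnPoint2, while SpawnPoint4 sits in a separate chain.
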(event `self.ReceiveBeginPlay`)

(fn `UserConstructionScript`)