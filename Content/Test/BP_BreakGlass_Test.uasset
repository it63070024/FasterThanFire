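; BP_BreakGlass_Test is a test breakable glass actor that can shatter when something overlaps its left or right trigger box.
; Each overlap rolls a roughly 30% chance, then a per-box DoOnce starts particles, Geometry Collection physics and a breaking sound.
; The right box also enables bomb physics on a child FS_BombField_Prototype field actor.
; Player damage and death-level logic exists but is never executed.
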(event `PlayGlassBreakSound`
  (`GameplayStatics.PlaySoundAtLocation` "/Game/BreakableGlass_v5/Sounds/Glass_Break_Cue.Glass_Break_Cue" (`self.K2_GetActorLocation`) (struct) 1.0 1.0 0.0 "/Game/Sound/NewSoundAttenuation.NewSoundAttenuation" null null null))

(event `self.Box_L.OnComponentBeginOverlap`
  (params (OverlappedComponent :type "PrimitiveComponent Object Reference") (OtherActor :type "Actor Object Reference") (OtherComp :type "PrimitiveComponent Object Reference") (OtherBodyIndex :type Integer) (bFromSweep :type Boolean) (SweepResult :type "HitResult Structure (by ref)"))
  (bind _geometrycollection (`self.GeometryCollection`))
  (if (<= (`KismetMathLibrary.RandomIntegerInRange` 0 100) 30)
    (`KismetSystemLibrary.PrintString` "Simulate")
    (`/Engine/EditorBlueprintResources/StandardMacros.DoOnce` false
      (:`Completed`
        (`ActorComponent.Activate` (`self.Glass_Break_PS`) false)
        (`PrimitiveComponent.SetSimulatePhysics` _geometrycollection true)
        (set `GeometryCollectionComponent.DamageThreshold` (`self.Damage Threshold`) _geometrycollection)
        (`self.PlayGlassBreakSound`)))))

(event `self.Box_R.OnComponentBeginOverlap`
  (params (OverlappedComponent :type "PrimitiveComponent Object Reference") (OtherActor :type "Actor Object Reference") (OtherComp :type "PrimitiveComponent Object Reference") (OtherBodyIndex :type Integer) (bFromSweep :type Boolean) (SweepResult :type "HitResult Structure (by ref)"))
  (bind _geometrycollection (`self.GeometryCollection`))
  (if (<= (`KismetMathLibrary.RandomIntegerInRange` 0 100) 30)
    (`KismetSystemLibrary.PrintString` "Simulate")
    (`/Engine/EditorBlueprintResources/StandardMacros.DoOnce` false
      (:`Completed`
        (`ActorComponent.Activate` (`self.Glass_Break_PS`) false)
        (`PrimitiveComponent.SetSimulatePhysics` _geometrycollection true)
        (set `GeometryCollectionComponent.DamageThreshold` (`self.Damage Threshold`) _geometrycollection)
        (bind _asfs_bomb_field_prototype (cast `/Engine/EditorResources/FieldNodes/FS_BombField_Prototype` (`ChildActorComponent.ChildActor` (`self.FS_BombField_Prototype`))))
        (`KismetSystemLibrary.PrintString` "pass")
        (set `/Engine/EditorResources/FieldNodes/FS_BombField_Prototype.useBomb` true _asfs_bomb_field_prototype)
        (set `/Engine/EditorResources/FieldNodes/FS_BombField_Prototype.useBombPhysics` true _asfs_bomb_field_prototype)
        (`self.PlayGlassBreakSound`)))))

(event `self.ReceiveTick`
  (params (DeltaSeconds :type "Float (single-precision)"))
  (if (`self.break`)
    _))

(fn `UserConstructionScript`)