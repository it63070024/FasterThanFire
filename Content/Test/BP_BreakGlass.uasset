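; Breakable glass hazard actor that can shatter on overlap and hurt the VR player.
; Either side box has a roughly 30% chance to trigger particles, sound and Geometry Collection fracture, destroying its cube while a Timeline moves the opposite one.
; Tick forces opposing velocities on both cubes until the Timeline ends and sets Break.
; It then damages the first VRPawn once, opening the Dead level with a cause of death if health runs out.
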(event `PlayGlassBreakSound`
  (`GameplayStatics.PlaySoundAtLocation` "/Game/BreakableGlass_v5/Sounds/Glass_Break_Cue.Glass_Break_Cue" (`self.K2_GetActorLocation`) (struct) 1.0 1.0 0.0 "/Game/Sound/NewSoundAttenuation.NewSoundAttenuation" null null null))

(event `self.Box_L.OnComponentBeginOverlap`
  (params (OverlappedComponent :type "PrimitiveComponent Object Reference") (OtherActor :type "Actor Object Reference") (OtherComp :type "PrimitiveComponent Object Reference") (OtherBodyIndex :type Integer) (bFromSweep :type Boolean) (SweepResult :type "HitResult Structure (by ref)"))
  (bind _geometrycollection (`self.GeometryCollection`))
  (bind _cube_r (`self.Cube_R`))
  (if (<= (`KismetMathLibrary.RandomIntegerInRange` 0 100) 30)
    (`KismetSystemLibrary.PrintString` "Simulate")
    (`/Engine/EditorBlueprintResources/StandardMacros.DoOnce` false
      (:`Completed`
        (`ActorComponent.Activate` (`self.Glass_Break_PS`) false)
        (`ActorComponent.K2_DestroyComponent` (`self.Cube_L`))
        (`PrimitiveComponent.SetSimulatePhysics` _geometrycollection true)
        (set `GeometryCollectionComponent.DamageThreshold` (`self.Damage Threshold`) _geometrycollection)
        (`PrimitiveComponent.SetSimulatePhysics` _cube_r true)
        (`self.PlayGlassBreakSound`)
        (bind (_direction _newtrack_0) (`Timeline|Timeline_0`)
          (:`Update`
            (`SceneComponent.K2_AddWorldTransform` _cube_r (`KismetMathLibrary.MakeTransform` (`KismetMathLibrary.MakeVector` (.x _newtrack_0))) false false))
          (:`Finished`
            (`ActorComponent.K2_DestroyComponent` _cube_r)
            (set `self.break` true :!label _label)
            (`/Engine/EditorBlueprintResources/StandardMacros.DoOnce` false
              (:`Completed`
                (bind _outactors (`GameplayStatics.GetAllActorsOfClass` "/Game/VRTemplate/Blueprints/VRPawn.VRPawn_C"))
                (bind _output (`|GetArrayItem` _outactors))
                (bind _playercurrenthealth (`/Game/VRTemplate/Blueprints/VRPawn.PlayerCurrentHealth` _output))
                (set `/Game/VRTemplate/Blueprints/VRPawn.PlayerCurrentHealth` (- _playercurrenthealth 15.0) _output)
                (if (<= _playercurrenthealth 0.0)
                  (bind _asftfinstance (cast `/Game/Widget/FTFInstance` (`GameplayStatics.GetGameInstance`)))
                  (set `/Game/Widget/FTFInstance.CauseOfDeath` "คุณเสียชืวิตจากการโดนแรงกระแทกจากเศษกระจก" _asftfinstance)
                  (`GameplayStatics.OpenLevel` "Dead"))))))))))

(event `self.Box_R.OnComponentBeginOverlap`
  (params (OverlappedComponent :type "PrimitiveComponent Object Reference") (OtherActor :type "Actor Object Reference") (OtherComp :type "PrimitiveComponent Object Reference") (OtherBodyIndex :type Integer) (bFromSweep :type Boolean) (SweepResult :type "HitResult Structure (by ref)"))
  (bind _geometrycollection (`self.GeometryCollection`))
  (if (<= (`KismetMathLibrary.RandomIntegerInRange` 0 100) 30)
    (`KismetSystemLibrary.PrintString` "Simulate")
    (`/Engine/EditorBlueprintResources/StandardMacros.DoOnce` false
      (:`Completed`
        (`ActorComponent.Activate` (`self.Glass_Break_PS`) false)
        (`ActorComponent.K2_DestroyComponent` (`self.Cube_R`))
        (`PrimitiveComponent.SetSimulatePhysics` _geometrycollection true)
        (set `GeometryCollectionComponent.DamageThreshold` (`self.Damage Threshold`) _geometrycollection)
        (`PrimitiveComponent.SetSimulatePhysics` (`self.Cube_L`) true)
        (`self.PlayGlassBreakSound`)
        (bind (_direction _newtrack_0) (`Timeline|Timeline`)
          (:`Update`
            (`SceneComponent.K2_AddWorldTransform` (`self.Cube_L`) (`KismetMathLibrary.MakeTransform` (`KismetMathLibrary.MakeVector` (.x _newtrack_0))) false false))
          (:`Finished`
            (`ActorComponent.K2_DestroyComponent` (`self.Cube_L`))
            (goto _label)))))))

(event `self.ReceiveTick`
  (params (DeltaSeconds :type "Float (single-precision)"))
  (if (not (`self.break`))
    (`PrimitiveComponent.SetPhysicsLinearVelocity` (`self.Cube_L`) (-900.0 0.0 0.0) false "None")
    (`PrimitiveComponent.SetPhysicsLinearVelocity` (`self.Cube_R`) (900.0 -0.0 -0.0) false "None")))

(fn `UserConstructionScript`)