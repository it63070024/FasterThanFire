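; BP_Evac_Sign_2 is a placeable evacuation sign for the fire-fighting systems set, configured entirely in the construction script.
; A decal selector picks one of three sign designs in an emissive or normal variant based on LightOn.
; A dynamic material instance then drives emissive strength when lit and optional mirroring.
; Optional CeilingSnap traces along the actor's up vector and moves the sign to the hit point.
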(fn `UserConstructionScript`
  (bind _decal_selector (`self.Decal Selector`))
  (bind _returnvalue (`SceneComponent.K2_GetComponentLocation` (`self.Sign`)))
  (`|ExecutionSequence`
    (:`then_0`
      ;[0.4582 1 0.5302] Decal Selector
      (if (`self.Light On`)
        (bind _output_get (set `self.Decals_Emissive` (`|MakeArray` "/Game/Fire_Fighting_Systems/Materials/Decal_MIs/MI_D_Evac_Sign_1.MI_D_Evac_Sign_1" "/Game/Fire_Fighting_Systems/Materials/Decal_MIs/MI_D_Evac_Sign_2.MI_D_Evac_Sign_2" "/Game/Fire_Fighting_Systems/Materials/Decal_MIs/MI_D_Evac_Sign_3.MI_D_Evac_Sign_3" :!type "MaterialInstance Object Reference")))
        (`DecalComponent.SetDecalMaterial` (`self.Decal`) (`|GetArrayItem` _output_get _decal_selector))
        (else
          (bind _output_get_2 (set `self.Decals_Normal` (`|MakeArray` "/Game/Fire_Fighting_Systems/Materials/Decal_MIs/MI_D_Evac_Sign_1_2.MI_D_Evac_Sign_1_2" "/Game/Fire_Fighting_Systems/Materials/Decal_MIs/MI_D_Evac_Sign_2_2.MI_D_Evac_Sign_2_2" "/Game/Fire_Fighting_Systems/Materials/Decal_MIs/MI_D_Evac_Sign_3_2.MI_D_Evac_Sign_3_2" :!type "MaterialInstance Object Reference")))
          (`DecalComponent.SetDecalMaterial` (`self.Decal`) (`|GetArrayItem` _output_get_2 _decal_selector))))
      (bind _returnvalue_2 (`DecalComponent.CreateDynamicMaterialInstance` (`self.Decal`)))
      (set `self.Sign Material` _returnvalue_2))
    (:`then_1`
      ;[1 0.06921 0.01945] Automatic Snap to Ceiling
      (if (`self.Ceiling Snap`)
        (bind (_outhit _returnvalue_3) (`KismetSystemLibrary.LineTraceSingle` _returnvalue (+ _returnvalue (* (`self.GetActorUpVector`) 100.0)) "TraceTypeQuery1"))
        (if _returnvalue_3
          (`SceneComponent.K2_SetWorldLocation` (`self.Sign`) (`.Location` (`GameplayStatics.BreakHitResult` _outhit)) false false))))
    (:`then_2`
      ;[0.2083 0.2432 1] Emissive Settings - Dynamic Material
      (if (`self.Light On`)
        (`MaterialInstanceDynamic.SetScalarParameterValue` (`self.Sign Material`) "Emissive Strength" (`self.Emissive`))))
    (:`then_3`
      ;[1 1 1] Mirror Decal
      (if (`self.Mirror Decal`)
        (`MaterialInstanceDynamic.SetScalarParameterValue` (`self.Sign Material`) "Mirror" -1.0)))))