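; BP_Ext_Cabinet_1 is a configurable fire extinguisher cabinet prop with no runtime logic.
; Its construction script picks one of two cabinet materials through MaterialSelector, then creates a dynamic material instance from it.
; Exposed dirt and dust settings for opacity, roughness, contrast and color feed that instance, so each placed cabinet can be weathered individually.
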(fn `UserConstructionScript`
  (bind _material (`self.Material`))
  (bind _material_2 (`self.Material`))
  (`|ExecutionSequence`
    (:`then_0`
      ;[0.6458 0.138 0.1278] Material Selector
      (`PrimitiveComponent.SetMaterial` (`self.Cabinet`) 0 (`|GetArrayItem` (`|MakeArray` "/Game/Fire_Fighting_Systems/Materials/MI_Ext_Cabinet_1_1.MI_Ext_Cabinet_1_1" "/Game/Fire_Fighting_Systems/Materials/MI_Ext_Cabinet_1_2.MI_Ext_Cabinet_1_2" :!type "MaterialInterface Object Reference") (`self.Material Selector`))))
    (:`then_1`
      ;[1 0.7492 0.1374] Dirt Settings
      (bind _returnvalue (`PrimitiveComponent.CreateDynamicMaterialInstance` (`self.Cabinet`) 0 null))
      (bind _output_get (set `self.Material` _returnvalue))
      (`MaterialInstanceDynamic.SetScalarParameterValue` _output_get "Dirt Opacity" (`self.Dirt Opacity`))
      (`MaterialInstanceDynamic.SetScalarParameterValue` _material "Dirt Roughness" (`self.Dirt Roughness`))
      (`MaterialInstanceDynamic.SetScalarParameterValue` _material "Dirt Contrast" (`self.Dirt Contrast`))
      (`MaterialInstanceDynamic.SetVectorParameterValue` _material "Dirt Color" (`self.Dirt Color`)))
    (:`then_2`
      ;[0.1771 0.1771 0.1771] Dust Settings
      (`MaterialInstanceDynamic.SetScalarParameterValue` _material_2 "Dust Opacity" (`self.Dust Opacity`))
      (`MaterialInstanceDynamic.SetScalarParameterValue` _material_2 "Dust Roughness" (`self.Dust Roughness`))
      (`MaterialInstanceDynamic.SetScalarParameterValue` _material_2 "Dust Contrast" (`self.Dust Contrast`))
      (`MaterialInstanceDynamic.SetVectorParameterValue` _material_2 "Dust Color" (`self.Dust Color`)))))