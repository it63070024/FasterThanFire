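; BP_W_Pipes_1 is a configurable pipe piece for fire fighting systems, set up entirely in the Construction Script with no active gameplay logic.
; It picks the static mesh from the Components selection and the material from an indexed array.
; A dynamic material instance then receives the color, dirt and dust overrides.
; An optional scale override resizes the mesh uniformly or only on X and Z when Y is locked.
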(fn `UserConstructionScript`
  (locals (sMeshes_Pipes :type "Array of StaticMesh Object Reference"))
  (bind _override_scale (`self.Override Scale`))
  (bind _scale (`self.Scale`))
  ;[0 0.4583 0.3653] Static Mesh Selector
  (`StaticMeshComponent.SetStaticMesh` (`self.Mesh_Pipes`) (`|GetArrayItem` (`local.sMeshes_Pipes`) (`KismetMathLibrary.Conv_ByteToInt` (`self.Components`))))
  (`|ExecutionSequence`
    (:`then_0`
      ;[1 0.1427 0.2124] Material Selector
      (`PrimitiveComponent.SetMaterial` (`self.Mesh_Pipes`) 0 (`|GetArrayItem` (`self.Pipe_Material`) (`self.Material Selector`))))
    (:`then_1`
      ;[0.1188 0.5162 1] Override Base Color
      (bind _returnvalue (`PrimitiveComponent.CreateDynamicMaterialInstance` (`self.Mesh_Pipes`) 0 null))
      (bind _output_get (set `self.Material` _returnvalue))
      (`MaterialInstanceDynamic.SetVectorParameterValue` _output_get "Color" (`self.Main Color`)))
    (:`then_2`
      ;[0.4583 0.378 0.1241] Dirt Settings
      (`MaterialInstanceDynamic.SetScalarParameterValue` (`self.Material`) "Dirt Opacity" (`self.Dirt Opacity`))
      (`MaterialInstanceDynamic.SetScalarParameterValue` (`self.Material`) "Dirt Roughness" (`self.Dirt Roughness`))
      (`MaterialInstanceDynamic.SetScalarParameterValue` (`self.Material`) "Dirt Contrast" (`self.Dirt Contrast`))
      (`MaterialInstanceDynamic.SetVectorParameterValue` (`self.Material`) "Dirt Color" (`self.Dirt Color`)))
    (:`then_3`
      ;[0.1458 0.1458 0.1458] Dust Settings
      (`MaterialInstanceDynamic.SetScalarParameterValue` (`self.Material`) "Dust Opacity" (`self.Dust Opacity`))
      (`MaterialInstanceDynamic.SetScalarParameterValue` (`self.Material`) "Dust Roughness" (`self.Dust Roughness`))
      (`MaterialInstanceDynamic.SetScalarParameterValue` (`self.Material`) "Dust Contrast" (`self.Dust Contrast`))
      (`MaterialInstanceDynamic.SetVectorParameterValue` (`self.Material`) "Dust Color" (`self.Dust Color`)))
    (:`then_4`
      ;[0.1645 1 0.2462] Override Scale
      (if (`self.Lock Y axis scale`)
        (if _override_scale
          (`SceneComponent.SetWorldScale3D` (`self.Mesh_Pipes`) (`KismetMathLibrary.MakeVector` _scale 1.0 _scale))
          (else
            (`SceneComponent.SetWorldScale3D` (`self.Mesh_Pipes`) (1.0 1.0 1.0) :!label _label)))
        (elif _override_scale
          (`SceneComponent.SetWorldScale3D` (`self.Mesh_Pipes`) (`KismetMathLibrary.MakeVector` _scale _scale _scale))
          (else
            (goto _label)))))))