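; BP_Hydrant_3 is a fire hydrant prop, customizable per instance, with no active gameplay logic.
; Its construction script applies a selected pipe material to the base, flange, pipe extension and both elbow meshes.
; It then creates dynamic material instances on those meshes to override main color and tune dirt and dust opacity, roughness, contrast and color.
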(fn `UserConstructionScript`
  (bind _material (`self.Material`))
  (bind _material_2 (`self.Material`))
  (`|ExecutionSequence`
    (:`then_0`
      ;[0.7708 0.1114 0.1044] Material Selector
      (bind _output_get (set `self.Editable Meshes` (`|MakeArray` (`self.base`) (`self.Flange`) (`self.Pipe_Extension`) (`self.Elbow_L`) (`self.Elbow_R`))))
      (for _array_element _output_get
        (`PrimitiveComponent.SetMaterial` _array_element 0 (`|GetArrayItem` (`self.Pipe_Material`) (`self.Material Selector`)))))
    (:`then_1`
      ;[0.1705 0.5122 1] Override Main Color
      (for _array_element_2 (`self.Editable Meshes`)
        (bind _returnvalue (`PrimitiveComponent.CreateDynamicMaterialInstance` _array_element_2 0 null))
        (bind _output_get_2 (set `self.Material` _returnvalue))
        (`MaterialInstanceDynamic.SetVectorParameterValue` _output_get_2 "Color" (`self.Main Color`))
        ;[1 0.8927 0.2891] Dirt Settings
        (`MaterialInstanceDynamic.SetScalarParameterValue` _material "Dirt Opacity" (`self.Dirt Opacity`))
        (`MaterialInstanceDynamic.SetScalarParameterValue` _material "Dirt Roughness" (`self.Dirt Roughness`))
        (`MaterialInstanceDynamic.SetScalarParameterValue` _material "Dirt Contrast" (`self.Dirt Contrast`))
        (`MaterialInstanceDynamic.SetVectorParameterValue` _material "Dirt Color" (`self.Dirt Color`))
        ;[0.1302 0.1302 0.1302] Dust Settings
        (`MaterialInstanceDynamic.SetScalarParameterValue` _material_2 "Dust Opacity" (`self.Dust Opacity`))
        (`MaterialInstanceDynamic.SetScalarParameterValue` _material_2 "Dust Roughness" (`self.Dust Roughness`))
        (`MaterialInstanceDynamic.SetScalarParameterValue` _material_2 "Dust Contrast" (`self.Dust Contrast`))
        (`MaterialInstanceDynamic.SetVectorParameterValue` _material_2 "Dust Color" (`self.Dust Color`))))))