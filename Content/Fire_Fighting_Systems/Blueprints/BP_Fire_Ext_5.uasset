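; BP_Fire_Ext_5 is a fire extinguisher prop whose look is configured in the construction script, with no active gameplay logic.
; A selector index picks one of four material instances for the FireExt mesh.
; The script then creates a dynamic material instance from it and applies the tank color plus dirt and dust parameters for opacity, roughness, color and contrast.
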(fn `UserConstructionScript`
  (`|ExecutionSequence`
    (:`then_0`
      ;[1 0.228 0.2081] Material Selector
      (bind _output_get (set `self.Material` (`|MakeArray` "/Game/Fire_Fighting_Systems/Materials/MI_Fire_Ext_5_1.MI_Fire_Ext_5_1" "/Game/Fire_Fighting_Systems/Materials/MI_Fire_Ext_5_2.MI_Fire_Ext_5_2" "/Game/Fire_Fighting_Systems/Materials/MI_Fire_Ext_5_3.MI_Fire_Ext_5_3" "/Game/Fire_Fighting_Systems/Materials/MI_Fire_Ext_5_4.MI_Fire_Ext_5_4" :!type "MaterialInterface Object Reference")))
      (`PrimitiveComponent.SetMaterial` (`self.Fire_Ext`) 0 (`|GetArrayItem` _output_get (`self.Material Selector`))))
    (:`then_1`
      ;[0.2603 0.9901 1] Override Base Color
      (bind _returnvalue (`PrimitiveComponent.CreateDynamicMaterialInstance` (`self.Fire_Ext`) 0 null))
      (bind _output_get_2 (set `self.Ext Material` _returnvalue))
      (`MaterialInstanceDynamic.SetVectorParameterValue` _output_get_2 "Color" (`self.Tank Color`)))
    (:`then_2`
      ;[0.4583 0.2765 0.1101] Dirt Settings
      (`MaterialInstanceDynamic.SetScalarParameterValue` (`self.Ext Material`) "Dirt Opacity" (`self.Dirt Opacity`))
      (`MaterialInstanceDynamic.SetScalarParameterValue` (`self.Ext Material`) "Dirt Roughness" (`self.Dirt Roughness`))
      (`MaterialInstanceDynamic.SetVectorParameterValue` (`self.Ext Material`) "Dirt Color" (`self.Dirt Color`))
      (`MaterialInstanceDynamic.SetScalarParameterValue` (`self.Ext Material`) "Dirt Contrast" (`self.Dirt Contrast`)))
    (:`then_3`
      ;[0.1458 0.1458 0.1458] Dust Settings
      (`MaterialInstanceDynamic.SetScalarParameterValue` (`self.Ext Material`) "Dust Opacity" (`self.Dust Opacity`))
      (`MaterialInstanceDynamic.SetScalarParameterValue` (`self.Ext Material`) "Dust Roughness" (`self.Dust Roughness`))
      (`MaterialInstanceDynamic.SetVectorParameterValue` (`self.Ext Material`) "Dust Color" (`self.Dust Color`))
      (`MaterialInstanceDynamic.SetScalarParameterValue` (`self.Ext Material`) "Dust Contrast" (`self.Dust Contrast`)))))