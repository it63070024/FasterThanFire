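; BP_Evac_Sign_3 is an evacuation sign actor that displays one of five decal designs, configured entirely in the construction script.
; A selector index picks the decal material from an emissive set when the light is on, otherwise from a normal set.
; A dynamic material instance then receives the emissive strength for lit signs and an optional mirror flip.
; The event graph holds no active logic.
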(fn `UserConstructionScript`
  (bind _decal_selector (`self.Decal Selector`))
  (`|ExecutionSequence`
    (:`then_0`
      ;[0.4582 1 0.5302] Decal Selector
      (if (`self.Light On`)
        (bind _output_get (set `self.Decals_Emissive` (`|MakeArray` "/Game/Fire_Fighting_Systems/Materials/Decal_MIs/MI_D_Evac_Sign_1.MI_D_Evac_Sign_1" "/Game/Fire_Fighting_Systems/Materials/Decal_MIs/MI_D_Evac_Sign_2.MI_D_Evac_Sign_2" "/Game/Fire_Fighting_Systems/Materials/Decal_MIs/MI_D_Evac_Sign_3.MI_D_Evac_Sign_3" "/Game/Fire_Fighting_Systems/Materials/Decal_MIs/MI_D_Evac_Sign_4.MI_D_Evac_Sign_4" "/Game/Fire_Fighting_Systems/Materials/Decal_MIs/MI_D_Evac_Sign_5.MI_D_Evac_Sign_5" :!type "MaterialInstance Object Reference")))
        (`DecalComponent.SetDecalMaterial` (`self.Decal`) (`|GetArrayItem` _output_get _decal_selector))
        (else
          (bind _output_get_2 (set `self.Decals_Normal` (`|MakeArray` "/Game/Fire_Fighting_Systems/Materials/Decal_MIs/MI_D_Evac_Sign_1_2.MI_D_Evac_Sign_1_2" "/Game/Fire_Fighting_Systems/Materials/Decal_MIs/MI_D_Evac_Sign_2_2.MI_D_Evac_Sign_2_2" "/Game/Fire_Fighting_Systems/Materials/Decal_MIs/MI_D_Evac_Sign_3_2.MI_D_Evac_Sign_3_2" "/Game/Fire_Fighting_Systems/Materials/Decal_MIs/MI_D_Evac_Sign_4_2.MI_D_Evac_Sign_4_2" "/Game/Fire_Fighting_Systems/Materials/Decal_MIs/MI_D_Evac_Sign_5_2.MI_D_Evac_Sign_5_2" :!type "MaterialInstance Object Reference")))
          (`DecalComponent.SetDecalMaterial` (`self.Decal`) (`|GetArrayItem` _output_get_2 _decal_selector))))
      (bind _returnvalue (`DecalComponent.CreateDynamicMaterialInstance` (`self.Decal`)))
      (set `self.Sign Material` _returnvalue))
    (:`then_1`
      ;[0.2083 0.2432 1] Emissive Settings - Dynamic Material
      (if (`self.Light On`)
        (`MaterialInstanceDynamic.SetScalarParameterValue` (`self.Sign Material`) "Emissive Strength" (`self.Emissive`))))
    (:`then_2`
      ;[1 1 1] Mirror Decal
      (if (`self.Mirror Decal`)
        (`MaterialInstanceDynamic.SetScalarParameterValue` (`self.Sign Material`) "Mirror" -1.0)))))