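; Elevator hazard for a VR game that kills a player who stays inside by smoke suffocation.
; The Box trigger enables input so Use can open the doors, which slide via Open and Close timelines with an auto-close delay.
; The Dead trigger tracks whether the VRPawn is inside.
; If it is after a delay, Niagara activates, then the game instance receives a Thai cause-of-death message and the Dead level loads.
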(event `EnhancedInput|/Game/VRTemplate/Input/Actions/IA_Use`
  (params (ActionValue :type Boolean) (ElapsedSeconds :type "Float (double-precision)") (TriggeredSeconds :type "Float (double-precision)") (InputAction :type "InputAction Object Reference" :default "/Game/VRTemplate/Input/Actions/IA_Use.IA_Use"))
  (:`Started`
    (if (not (`self.Opening`))
      (`self.OpenDoor`)
      (`KismetSystemLibrary.Delay` 12.0)
      (if (`self.StayInside`)
        (`KismetSystemLibrary.PrintString` "that true")
        (`ActorComponent.Activate` (`self.Niagara`) false)
        (`KismetSystemLibrary.Delay` 8.0)
        (bind _asftfinstance (cast `/Game/Widget/FTFInstance` (`GameplayStatics.GetGameInstance`)))
        (set `/Game/Widget/FTFInstance.CauseOfDeath` "คุณขาดอากาศหายใจ เนื่องจากโดนรมควันในลิฟต์" _asftfinstance)
        (`GameplayStatics.OpenLevel` "Dead")))))

(event `self.Box.OnComponentBeginOverlap`
  (params (OverlappedComponent :type "PrimitiveComponent Object Reference") (OtherActor :type "Actor Object Reference") (OtherComp :type "PrimitiveComponent Object Reference") (OtherBodyIndex :type Integer) (bFromSweep :type Boolean) (SweepResult :type "HitResult Structure (by ref)"))
  (`self.EnableInput` (`GameplayStatics.GetPlayerController` 0)))

(event `OpenDoor`
  (bind _l_door (`self.L_door`))
  (bind _r_door (`self.R_door`))
  (bind _l_door_2 (`self.L_door`))
  (bind _r_door_2 (`self.R_door`))
  (bind (_relativelocation_x _relativelocation_y _relativelocation_z) (`KismetMathLibrary.BreakVector` (`SceneComponent.RelativeLocation` _l_door_2)))
  (bind (_relativelocation_x_2 _relativelocation_y_2 _relativelocation_z_2) (`KismetMathLibrary.BreakVector` (`SceneComponent.RelativeLocation` _r_door_2)))
  (bind (_relativelocation_x_3 _relativelocation_y_3 _relativelocation_z_3) (`KismetMathLibrary.BreakVector` (`SceneComponent.RelativeLocation` _l_door)))
  (bind (_relativelocation_x_4 _relativelocation_y_4 _relativelocation_z_4) (`KismetMathLibrary.BreakVector` (`SceneComponent.RelativeLocation` _r_door)))
  (set `self.Opening` true)
  (bind (_direction _newtrack_0) (`Timeline|open` :!via `PlayFromStart`)
    (:`Update`
      (`SceneComponent.K2_SetRelativeLocation` _l_door (`KismetMathLibrary.MakeVector` _relativelocation_x_3 _newtrack_0 _relativelocation_z_3) false false)
      (`SceneComponent.K2_SetRelativeLocation` _r_door (`KismetMathLibrary.MakeVector` _relativelocation_x_4 (* _newtrack_0 -1.0) _relativelocation_z_4) false false)
      (`KismetSystemLibrary.Delay` 6.0)
      (bind (_direction_2 _newtrack_0_2) (`Timeline|close` :!via `PlayFromStart`)
        (:`Update`
          (`SceneComponent.K2_SetRelativeLocation` _l_door_2 (`KismetMathLibrary.MakeVector` _relativelocation_x _newtrack_0_2 _relativelocation_z) false false)
          (`SceneComponent.K2_SetRelativeLocation` _r_door_2 (`KismetMathLibrary.MakeVector` _relativelocation_x_2 (* _newtrack_0_2 -1.0) _relativelocation_z_2) false false)
          (set `self.Opening` false))))))

(event `self.Box.OnComponentEndOverlap`
  (params (OverlappedComponent :type "PrimitiveComponent Object Reference") (OtherActor :type "Actor Object Reference") (OtherComp :type "PrimitiveComponent Object Reference") (OtherBodyIndex :type Integer))
  (`self.DisableInput` (`GameplayStatics.GetPlayerController` 0)))

(event `self.Dead.OnComponentBeginOverlap`
  (params (OverlappedComponent :type "PrimitiveComponent Object Reference") (OtherActor :type "Actor Object Reference") (OtherComp :type "PrimitiveComponent Object Reference") (OtherBodyIndex :type Integer) (bFromSweep :type Boolean) (SweepResult :type "HitResult Structure (by ref)"))
  (cast `/Game/VRTemplate/Blueprints/VRPawn` OtherActor)
  (set `self.StayInside` true)
  (`KismetSystemLibrary.PrintString` "Inside"))

(event `self.Dead.OnComponentEndOverlap`
  (params (OverlappedComponent :type "PrimitiveComponent Object Reference") (OtherActor :type "Actor Object Reference") (OtherComp :type "PrimitiveComponent Object Reference") (OtherBodyIndex :type Integer))
  (cast `/Game/VRTemplate/Blueprints/VRPawn` OtherActor)
  (set `self.StayInside` false)
  (`KismetSystemLibrary.PrintString` "outside"))

(fn `UserConstructionScript`)