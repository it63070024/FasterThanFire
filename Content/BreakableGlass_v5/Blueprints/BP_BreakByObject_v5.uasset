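; Temporary component that lets a moving physics object break BP_BreakableGlass_v5 panes along its path.
; On setup it optionally adds a bounds-sized sphere blocking Destructibles, then self-destroys after its lifetime.
; A per-tick Delay loop sphere-traces along the velocity, passing velocity-scaled hits to glass locally or through BreakOnServer when replicated.
; Tracing pauses after a hit until WaitForHit or WaitForServer ignores that pane and resumes.
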(event `BreakableGlassObjectEvent`
  (params (BreakableGlassChannel :type "EObjectTypeQuery Enum" :default "ObjectTypeQuery7") (Component :type "PrimitiveComponent Object Reference") (CreatePhysicsSphereCollision :type Boolean :default true) (`Component Lifetime (Seconds)` :type "Float (double-precision)" :default 5.0) (BreakRadius :type "Float (double-precision)" :default 20.0) (ImpulseForce :type "Float (double-precision)" :default 1.0) (AngularImpulse :type "Float (double-precision)" :default 1.0) (DrawDebugImpactRadius :type Boolean) (BreakOnServer :type "/Game/BreakableGlass_v5/Blueprints/BP_BreakOnServer_v5 Object Reference"))
  (set `self.CollisionObjectType` (`|MakeArray` BreakableGlassChannel))
  (bind _output_get (set `self.Component` Component))
  (set `self.Sphere Bound` (`.SphereRadius` (`KismetSystemLibrary.GetComponentBounds` _output_get)))
  (set `self.Component Lifetime` `Component Lifetime (Seconds)`)
  (set `self.BreakRadius` BreakRadius)
  (set `self.ImpulseForce` ImpulseForce)
  (set `self.AngularImpulse` AngularImpulse)
  (set `self.Draw Debug Impact Radius` DrawDebugImpactRadius)
  (set `self.Break on Server` BreakOnServer)
  (if CreatePhysicsSphereCollision
    (bind _returnvalue (`|AddComponentByClass` :`self` (`self.GetOwner`) :`Class` "/Script/Engine.SphereComponent"))
    (bind _output_get_2 (set `self.SphereBounds` _returnvalue))
    (`SphereComponent.SetSphereRadius` _output_get_2 (`self.Sphere Bound`) false)
    (`PrimitiveComponent.SetCollisionEnabled` _output_get_2 "QueryAndPhysics")
    (`PrimitiveComponent.SetCollisionObjectType` _output_get_2 "ECC_PhysicsBody")
    (`PrimitiveComponent.SetCollisionResponseToAllChannels` _output_get_2 "ECR_Ignore")
    (`PrimitiveComponent.SetCollisionResponseToChannel` _output_get_2 "ECC_Destructible" "ECR_Block"))
  (`KismetArrayLibrary.Array_Clear` (`self.LastHitActor`))
  (`self.Reset`)
  (`KismetSystemLibrary.Delay` (`self.Component Lifetime`))
  (`self.K2_DestroyComponent`))

(event `Reset`
  (bind _angularimpulse (`self.AngularImpulse`))
  (bind _breakradius (`self.BreakRadius`))
  (bind _sphere_bound (`self.Sphere Bound`))
  (bind _lasthitactor (`self.LastHitActor`))
  (bind _break_on_server (`self.Break on Server`))
  (bind _as_bp_breakable_glass_v_5 (`self.As BP Breakable Glass V 5`))
  (bind _returnvalue (* (`self.Launch Velocity`) (`self.ImpulseForce`)))
  (bind _returnvalue_2 (`KismetMathLibrary.VSize` (`self.Launch Velocity`)))
  (bind _returnvalue_3 (`SceneComponent.K2_GetComponentLocation` (`self.Component`)))
  (bind _returnvalue_4 (`PrimitiveComponent.GetPhysicsLinearVelocity` (`self.Component`) "None"))
  (set `self.Launch Velocity` _returnvalue_4)
  (`KismetArrayLibrary.Array_Append` _lasthitactor (`|MakeArray` (`self.GetOwner`)))
  (bind _outhit (`KismetSystemLibrary.SphereTraceSingleForObjects` (`KismetMathLibrary.SelectVector` (`self.Trace End`) _returnvalue_3 (`self.Pick A`)) (+ _returnvalue_3 (`KismetMathLibrary.Vector_ClampSizeMax` _returnvalue_4 (+ (`self.Sphere Bound`) 20.0))) (`self.Sphere Bound`) (`self.CollisionObjectType`) false _lasthitactor))
  (set `self.Trace End` (`.TraceEnd` (`GameplayStatics.BreakHitResult` _outhit)))
  (set `self.Pick A` true)
  (if (== (`GameplayStatics.GetObjectClass` (`.HitActor` (`GameplayStatics.BreakHitResult` _outhit))) "/Game/BreakableGlass_v5/Blueprints/BP_BreakableGlass_v5.BP_BreakableGlass_v5_C")
    (bind _asbp_breakable_glass_v_5 (cast `/Game/BreakableGlass_v5/Blueprints/BP_BreakableGlass_v5` (`.HitActor` (`GameplayStatics.BreakHitResult` _outhit)))
      (:`then`
        (bind _output_get (set `self.As BP Breakable Glass V 5` _asbp_breakable_glass_v_5))
        (`/Game/BreakableGlass_v5/Blueprints/BP_BreakableGlass_v5.Set Object Ref` _output_get self)
        (set `self.Trace End` (`.ImpactPoint` (`GameplayStatics.BreakHitResult` _outhit)))
        (if (`/Game/BreakableGlass_v5/Blueprints/BP_BreakableGlass_v5.Replicate Multicast ( BETA )` _output_get)
          (`/Engine/EditorBlueprintResources/StandardMacros.IsValid` _break_on_server
            (:`Is Valid`
              (`/Game/BreakableGlass_v5/Blueprints/BP_BreakOnServer_v5.CallBreakOnServer` _break_on_server _as_bp_breakable_glass_v_5 (`.ImpactPoint` (`GameplayStatics.BreakHitResult` _outhit)) _returnvalue _angularimpulse _breakradius 0.0 _sphere_bound _returnvalue_2 "NewEnumerator1"))
            (:`Is Not Valid`
              (`/Game/BreakableGlass_v5/Blueprints/BP_BreakableGlass_v5.HIT LOCAL` _as_bp_breakable_glass_v_5 (`.ImpactPoint` (`GameplayStatics.BreakHitResult` _outhit)) _returnvalue _angularimpulse _breakradius 0.0 _sphere_bound _returnvalue_2 "NewEnumerator1" :!label _label)))
          (else
            (goto _label))))
      (:`CastFailed`
        (`KismetSystemLibrary.Delay` 0.0 :!label _label_2)
        (`self.Reset`)))
    (else
      (goto _label_2))))

(event `Wait For Server`
  ;[1 1 1] Response Hit
  (`KismetArrayLibrary.Array_Add` (`self.LastHitActor`) (`self.As BP Breakable Glass V 5`) :!label _label_3)
  (if (`self.Draw Debug Impact Radius`)
    (`KismetSystemLibrary.DrawDebugSphere` (`self.Trace End`) (`self.BreakRadius`) 16 (struct :`R` 1.0 :`A` 1.0) 10.0 0.2))
  (`self.Reset`))

(event `Wait For Hit`
  ;[1 1 1] Response Hit
  (goto _label_3))