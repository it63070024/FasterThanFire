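; Component that breaks BP_BreakableGlass_v5 panes within a spherical force field around its owning actor.
; BreakableGlassForceFieldEvent stores the passed settings, sphere-traces the glass channel and scales each pane's impact radius and outward impulse by distance.
; Hits route through the BreakOnServer reference for replicated glass when valid, otherwise through HITLOCAL.
; Each pane receives a reference to this component, whose WaitForServer and WaitForHit events optionally draw the debug radius.
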(event `WaitForServer`
  (if (`self.DrawDebugForceFieldRadius`) :!label _label
    (`KismetSystemLibrary.DrawDebugSphere` (`Actor.K2_GetActorLocation` (`self.GetOwner`)) (`self.ForceFieldRadius`) 32 (struct :`R` 1.0 :`G` 1.0 :`B` 1.0 :`A` 1.0) 2.0 1.0)))

(event `WaitForHit`
  (goto _label))

(event `BreakableGlassForceFieldEvent`
  (params (BreakableGlassChannel :type "EObjectTypeQuery Enum" :default "ObjectTypeQuery7") (BreakFromCenter :type Boolean) (ForceFieldRadius :type "Float (double-precision)" :default 500.0) (`MinRadiusAtDistance ` :type "Float (double-precision)" :default 20.0) (`MaxRadiusAtDistance ` :type "Float (double-precision)" :default 100.0) (MinImpulse :type "Float (double-precision)" :default 1000.0) (MaxImpulse :type "Float (double-precision)" :default 5000.0) (AngularImpulse :type "Float (double-precision)" :default 1.0) (DrawDebugForceFieldRadius :type Boolean) (BreakOnServer :type "/Game/BreakableGlass_v5/Blueprints/BP_BreakOnServer_v5 Object Reference"))
  (bind _outradius (`self.OutRadius`))
  (bind _as_bp_breakable_glass_v_5 (`self.As BP Breakable Glass V 5`))
  (bind _linearvelocity (`self.LinearVelocity`))
  (bind _angularimpulse (`self.AngularImpulse`))
  (bind _as_bp_breakable_glass_v_5_2 (`self.As BP Breakable Glass V 5`))
  (bind _break_on_server (`self.Break on Server`))
  (bind _returnvalue (`Actor.K2_GetActorLocation` (`self.GetOwner`)))
  (bind _returnvalue_2 (`Actor.K2_GetActorLocation` (`self.GetOwner`)))
  (bind _returnvalue_3 (`KismetMathLibrary.SelectVector` (`Actor.K2_GetActorLocation` _as_bp_breakable_glass_v_5) (`self.Hit Position`) (`self.BreakFromCenter`)))
  (set `self.CollisionObjectType` (`|MakeArray` BreakableGlassChannel))
  (set `self.BreakFromCenter` BreakFromCenter)
  (set `self.ForceFieldRadius` ForceFieldRadius)
  (set `self.MinRadiusAtDistance ` `MinRadiusAtDistance `)
  (set `self.MaxRadiusAtDistance ` `MaxRadiusAtDistance `)
  (set `self.MinImpulse` MinImpulse)
  (set `self.MaxImpulse` MaxImpulse)
  (set `self.AngularImpulse` AngularImpulse)
  (set `self.DrawDebugForceFieldRadius` DrawDebugForceFieldRadius)
  (set `self.Break on Server` BreakOnServer)
  (bind _outhits (`KismetSystemLibrary.SphereTraceMultiForObjects` _returnvalue_2 _returnvalue_2 (`self.ForceFieldRadius`) (`self.CollisionObjectType`) false (`|MakeArray` (`self.GetOwner`))))
  (for _array_element _outhits
    (if (== (`GameplayStatics.GetObjectClass` (`.HitActor` (`GameplayStatics.BreakHitResult` _array_element))) "/Game/BreakableGlass_v5/Blueprints/BP_BreakableGlass_v5.BP_BreakableGlass_v5_C")
      (bind _asbp_breakable_glass_v_5 (cast `/Game/BreakableGlass_v5/Blueprints/BP_BreakableGlass_v5` (`.HitActor` (`GameplayStatics.BreakHitResult` _array_element))))
      (bind _output_get (set `self.As BP Breakable Glass V 5` _asbp_breakable_glass_v_5))
      (`/Game/BreakableGlass_v5/Blueprints/BP_BreakableGlass_v5.Set ForceField Ref` _output_get self)
      (set `self.Hit Position` (`.ImpactPoint` (`GameplayStatics.BreakHitResult` _array_element)))
      (bind _returnvalue_4 (`Actor.K2_GetActorLocation` (`.HitActor` (`GameplayStatics.BreakHitResult` _array_element))))
      (bind _returnvalue_5 (`KismetMathLibrary.Vector_Distance` _returnvalue_4 _returnvalue))
      (set `self.OutRadius` (`KismetMathLibrary.MapRangeClamped` _returnvalue_5 (`self.ForceFieldRadius`) 0.0 (`self.MinRadiusAtDistance `) (* (`KismetMathLibrary.FMax` (`/Game/BreakableGlass_v5/Blueprints/BP_BreakableGlass_v5.Scale Y` _output_get) (`/Game/BreakableGlass_v5/Blueprints/BP_BreakableGlass_v5.Scale Z` _output_get)) (`self.MaxRadiusAtDistance `))))
      (set `self.LinearVelocity` (* (`KismetMathLibrary.GetDirectionUnitVector` _returnvalue _returnvalue_4) (`KismetMathLibrary.MapRangeClamped` _returnvalue_5 (`self.ForceFieldRadius`) 0.0 (`self.MinImpulse`) (`self.MaxImpulse`))))
      (if (`/Game/BreakableGlass_v5/Blueprints/BP_BreakableGlass_v5.Replicate Multicast ( BETA )` _as_bp_breakable_glass_v_5)
        (`/Engine/EditorBlueprintResources/StandardMacros.IsValid` _break_on_server
          (:`Is Valid`
            (`/Game/BreakableGlass_v5/Blueprints/BP_BreakOnServer_v5.CallBreakOnServer` _break_on_server _as_bp_breakable_glass_v_5_2 _returnvalue_3 _linearvelocity _angularimpulse _outradius 0.0 1.0 1000000.0 "NewEnumerator3"))
          (:`Is Not Valid`
            (`/Game/BreakableGlass_v5/Blueprints/BP_BreakableGlass_v5.HIT LOCAL` _as_bp_breakable_glass_v_5_2 _returnvalue_3 _linearvelocity _angularimpulse _outradius 0.0 1.0 1000000.0 "NewEnumerator3" :!label _label_2)))
        (else
          (goto _label_2))))))