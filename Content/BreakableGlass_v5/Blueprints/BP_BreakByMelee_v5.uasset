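; Melee component that breaks BP_BreakableGlass_v5 actors struck by a weapon during a timed attack window or continuously.
; A self-repeating, frequency-limited sphere trace runs between two sockets, gated by animation duration unless EachFrame is set.
; Hits scale impulse by the traced component's physics velocity, then break glass through BreakOnServer when replication is enabled and valid, otherwise locally.
; Optional debug drawing shows traces and impact points.
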(event `Reset`
  (bind _returnvalue (`GameplayStatics.GetWorldDeltaSeconds`))
  (bind _break_on_server (`self.Break on Server`))
  (bind _angularimpulse (`self.AngularImpulse`))
  (bind _as_bp_breakable_glass_v_5 (`self.As BP Breakable Glass V 5`))
  (bind _impulseradius (`self.ImpulseRadius`))
  (bind _radius (`self.Radius`))
  (bind _freq (`self.Freq`))
  (bind _component (`self.Component`))
  (bind _returnvalue_2 (* (`self.LinearVelocity`) (`self.ImpulseForce`)))
  (bind _returnvalue_3 (/ 1.0 _returnvalue))
  (bind _returnvalue_4 (* _returnvalue (`KismetMathLibrary.FClamp` (/ _returnvalue_3 (`KismetMathLibrary.Conv_IntToDouble` (`KismetMathLibrary.Clamp` _freq 1 _freq))) 0.0 _returnvalue_3)))
  (if (not (`self.Each Frame`))
    (`/Engine/EditorBlueprintResources/StandardMacros.Gate` true :!label _label
      (:`Exit`
        _)))
  (bind _returnvalue_5 (`PrimitiveComponent.GetPhysicsLinearVelocity` (`self.Component`) "None" :!label _label_2))
  (set `self.LinearVelocity` _returnvalue_5)
  (bind _outhit (`KismetSystemLibrary.SphereTraceSingleForObjects` (`SceneComponent.GetSocketLocation` _component (`self.Start`)) (`SceneComponent.GetSocketLocation` _component (`self.End`)) (`self.Radius`) (`self.CollisionObjectType`) false (`|MakeArray` (`self.GetOwner`)) (select `bool` (stale `BreakableGlassMeleeEvent` DrawDebugTraceCapsule) :`true` "ForDuration" :!type "EDrawDebugTrace Enum") true (struct :`R` 1.0 :`A` 1.0) (struct :`G` 1.0 :`A` 1.0) _returnvalue_4))
  (if (== (`GameplayStatics.GetObjectClass` (`.HitActor` (`GameplayStatics.BreakHitResult` _outhit))) "/Game/BreakableGlass_v5/Blueprints/BP_BreakableGlass_v5.BP_BreakableGlass_v5_C")
    (bind _asbp_breakable_glass_v_5 (cast `/Game/BreakableGlass_v5/Blueprints/BP_BreakableGlass_v5` (`.HitActor` (`GameplayStatics.BreakHitResult` _outhit)))
      (:`then`
        (bind _output_get (set `self.As BP Breakable Glass V 5` _asbp_breakable_glass_v_5))
        (`/Game/BreakableGlass_v5/Blueprints/BP_BreakableGlass_v5.SetMelee Ref` _output_get self)
        (if (`/Game/BreakableGlass_v5/Blueprints/BP_BreakableGlass_v5.Replicate Multicast ( BETA )` _output_get)
          (`/Engine/EditorBlueprintResources/StandardMacros.IsValid` _break_on_server
            (:`Is Valid`
              (`/Game/BreakableGlass_v5/Blueprints/BP_BreakOnServer_v5.CallBreakOnServer` _break_on_server _as_bp_breakable_glass_v_5 (`.ImpactPoint` (`GameplayStatics.BreakHitResult` _outhit)) _returnvalue_2 _angularimpulse _impulseradius 0.0 _radius 1000000.0 "NewEnumerator4"))
            (:`Is Not Valid`
              (`/Game/BreakableGlass_v5/Blueprints/BP_BreakableGlass_v5.HIT LOCAL` _as_bp_breakable_glass_v_5 (`.ImpactPoint` (`GameplayStatics.BreakHitResult` _outhit)) _returnvalue_2 _angularimpulse _impulseradius 0.0 _radius 1000000.0 "NewEnumerator4" :!label _label_3)))
          (else
            (goto _label_3))))
      (:`CastFailed`
        _)))
  (`KismetSystemLibrary.Delay` _returnvalue_4)
  (`self.Reset`))

(event `BreakableGlassMeleeEvent`
  (params (CollisionObjectType :type "EObjectTypeQuery Enum" :default "ObjectTypeQuery7") (Component :type "PrimitiveComponent Object Reference") (SocketStartName :type Name) (SocketEndName :type Name) (ObjectRadius :type "Float (double-precision)" :default 10.0) (ImpulseRadius :type "Float (double-precision)" :default 10.0) (ImpulseForce :type "Float (double-precision)" :default 1.0) (AngularImpulse :type "Float (double-precision)" :default 1.0) (`Duration (Animation Time)` :type "Float (double-precision)" :default 1.0) (`Frequency(Hits per Second)` :type Integer :default 10) (EachFrame :type Boolean) (DrawDebugTraceCapsule :type Boolean) (BreakOnServer :type "/Game/BreakableGlass_v5/Blueprints/BP_BreakOnServer_v5 Object Reference"))
  (set `self.CollisionObjectType` (`|MakeArray` CollisionObjectType))
  (set `self.Component` Component)
  (set `self.Start` SocketStartName)
  (set `self.End` SocketEndName)
  (set `self.Radius` ObjectRadius)
  (set `self.ImpulseRadius` ImpulseRadius)
  (set `self.ImpulseForce` ImpulseForce)
  (set `self.AngularImpulse` AngularImpulse)
  (set `self.Break on Server` BreakOnServer)
  (set `self.Freq` `Frequency(Hits per Second)`)
  (bind _output_get (set `self.Each Frame` EachFrame))
  (if _output_get
    (goto _label_2)
    (else
      (`|ExecutionSequence`
        (:`then_0`
          (goto _label :!via `Open`))
        (:`then_1`
          (`KismetSystemLibrary.RetriggerableDelay` `Duration (Animation Time)`)
          (goto _label :!via `Close`))
        (:`then_2`
          (goto _label_2))))))

(event `WaitForServer`
  (bind _returnvalue (`GameplayStatics.GetWorldDeltaSeconds`))
  (bind _freq (`self.Freq`))
  (bind _returnvalue_2 (/ 1.0 _returnvalue))
  ;[1 1 1] Return Hit
  (if (stale `BreakableGlassMeleeEvent` DrawDebugTraceCapsule) :!label _label_4
    (`KismetSystemLibrary.DrawDebugSphere` (`.ImpactPoint` (`GameplayStatics.BreakHitResult` (stale `Reset` _outhit))) (`self.Radius`) 16 (struct :`R` 1.0 :`A` 1.0) (* _returnvalue (`KismetMathLibrary.FClamp` (/ _returnvalue_2 (`KismetMathLibrary.Conv_IntToDouble` (`KismetMathLibrary.Clamp` _freq 1 _freq))) 0.0 _returnvalue_2)) 0.2)))

(event `WaitForHit`
  ;[1 1 1] Return Hit
  (goto _label_4))