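; Component that lets its owning Character break BP_BreakableGlass_Mod panes by moving into them.
; An init event stores impulse settings and can add a physics capsule that blocks only Destructibles.
; A gated Tick capsule-traces along velocity, sending close hits to the glass locally or through BreakOnServer when replication is enabled.
; After a hit the gate stays closed until WaitForHit or WaitForServer reopens it following a frequency-based delay.
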(event `BreakableGlassCharacterEvent`
  (params (BreakableGlassChannel :type "EObjectTypeQuery Enum" :default "ObjectTypeQuery7") (CreatePhyisicCapsuleCollision :type Boolean :default true) (ImpuseForce :type "Float (double-precision)" :default 1.0) (`Angular impulse` :type "Float (double-precision)" :default 1.0) (`Frequency (HitsPerSecond)` :type Integer :default 10) (DrawDebugImpactCapsule :type Boolean) (BreakOnServer :type "/Game/BreakableGlass_v5/Blueprints/BP_BreakOnServer_v5 Object Reference"))
  (set `self.CollisionObjectType` (`|MakeArray` BreakableGlassChannel))
  (set `self.Freq` `Frequency (HitsPerSecond)`)
  (set `self.ImpuseForce` ImpuseForce)
  (set `self.Angular impulse` `Angular impulse`)
  (set `self.Break on Server` BreakOnServer)
  (set `self.Draw Debug Capsule` DrawDebugImpactCapsule)
  (bind _ascharacter (cast `Character` (`self.GetOwner`))
    (:`then`
      (bind _output_get (set `self.As Character` _ascharacter))
      (if CreatePhyisicCapsuleCollision
        (bind _returnvalue (`|AddComponentByClass` :`self` _output_get :`Class` "/Script/Engine.CapsuleComponent"))
        (bind _output_get_2 (set `self.Physic capsule` _returnvalue))
        (`PrimitiveComponent.SetCollisionEnabled` _output_get_2 "QueryAndPhysics")
        (`PrimitiveComponent.SetCollisionObjectType` _output_get_2 "ECC_PhysicsBody")
        (`PrimitiveComponent.SetCollisionResponseToAllChannels` _output_get_2 "ECR_Ignore")
        (`PrimitiveComponent.SetCollisionResponseToChannel` _output_get_2 "ECC_Destructible" "ECR_Block")
        (bind (_outradius _outhalfheight) (`CapsuleComponent.GetScaledCapsuleSize` (`Character.CapsuleComponent` _ascharacter)))
        (`CapsuleComponent.SetCapsuleSize` _output_get_2 _outradius _outhalfheight false)))
    (:`CastFailed`
      _))
  (set `self.Out Radius` _outradius)
  (set `self.Out Half Height` _outhalfheight)
  (`self.WaitForHit`))

(event `self.ReceiveTick`
  (params (DeltaSeconds :type "Float (single-precision)"))
  (bind _returnvalue (`GameplayStatics.GetWorldDeltaSeconds`))
  (bind _out_radius (`self.Out Radius`))
  (bind _angular_impulse (`self.Angular impulse`))
  (bind _break_on_server (`self.Break on Server`))
  (bind _out_half_height (`self.Out Half Height`))
  (bind _freq (`self.Freq`))
  (bind _as_character (`self.As Character`))
  (bind _hit_position (`self.Hit Position`))
  (bind _returnvalue_2 (`KismetMathLibrary.VSize` (`self.LinearVelocity`)))
  (bind _returnvalue_3 (* (`self.LinearVelocity`) (`self.ImpuseForce`)))
  (bind _returnvalue_4 (`Actor.K2_GetActorLocation` _as_character))
  (bind _returnvalue_5 (/ 1.0 _returnvalue))
  (`/Engine/EditorBlueprintResources/StandardMacros.Gate` true :!label _label
    (:`Exit`
      (`self.Close`)
      (bind _returnvalue_6 (`PrimitiveComponent.GetPhysicsLinearVelocity` (`Character.CapsuleComponent` _as_character) "None"))
      (bind _output_get (set `self.LinearVelocity` _returnvalue_6))
      (if (>= (`KismetMathLibrary.VSize` _output_get) 2.0)
        (bind _outhit (`KismetSystemLibrary.CapsuleTraceSingleForObjects` _returnvalue_4 (+ _returnvalue_4 (`KismetMathLibrary.Vector_ClampSizeMax` _output_get 100.0)) (`self.Out Radius`) (`self.Out Half Height`) (`self.CollisionObjectType`) false (`|MakeArray` _as_character :!type "Actor Object Reference") "None" true (struct :`R` 1.0 :`A` 1.0) (struct :`G` 1.0 :`A` 1.0) (`self.Frequency`)))
        (bind (_bblockinghit _binitialoverlap _time _distance _location _impactpoint _normal _impactnormal _physmat _hitactor) (`GameplayStatics.BreakHitResult` _outhit))
        (if (== (`GameplayStatics.GetObjectClass` _hitactor) "/Game/BreakableGlass_v5/Blueprints/BP_BreakableGlass_Mod.BP_BreakableGlass_Mod_C")
          (if (<= _distance 3.0)
            (bind _asbp_breakable_glass_mod (cast `/Game/BreakableGlass_v5/Blueprints/BP_BreakableGlass_Mod` _hitactor)
              (:`then`
                (`/Game/BreakableGlass_v5/Blueprints/BP_BreakableGlass_Mod.Set Character Ref` _asbp_breakable_glass_mod self)
                (set `self.Hit Position` _impactpoint)
                (set `self.Frequency` (* _returnvalue (`KismetMathLibrary.FClamp` (/ _returnvalue_5 (`KismetMathLibrary.Conv_IntToDouble` (`KismetMathLibrary.Clamp` _freq 1 _freq))) 0.0 _returnvalue_5)))
                (if (`/Game/BreakableGlass_v5/Blueprints/BP_BreakableGlass_Mod.Replicate Multicast ( BETA )` _asbp_breakable_glass_mod)
                  (`/Engine/EditorBlueprintResources/StandardMacros.IsValid` _break_on_server
                    (:`Is Valid`
                      (`/Game/BreakableGlass_v5/Blueprints/BP_BreakOnServer_v5.CallBreakOnServer` _break_on_server _asbp_breakable_glass_mod _hit_position _returnvalue_3 _angular_impulse _out_radius _out_half_height _out_radius _returnvalue_2 "NewEnumerator2"))
                    (:`Is Not Valid`
                      (`/Game/BreakableGlass_v5/Blueprints/BP_BreakableGlass_Mod.HIT LOCAL` _asbp_breakable_glass_mod _hit_position _returnvalue_3 _angular_impulse _out_radius _out_half_height _out_radius _returnvalue_2 "NewEnumerator2" :!label _label_2)))
                  (else
                    (goto _label_2))))
              (:`CastFailed`
                (`self.Open` :!label _label_3)))
            (else
              (goto _label_3)))
          (else
            (goto _label_3)))
        (else
          (goto _label_3))))))

(event `WaitForServer`
  (if (`self.Draw Debug Capsule`) :!label _label_4
    (`KismetSystemLibrary.DrawDebugCapsule` (`self.Hit Position`) (`self.Out Half Height`) (`self.Out Radius`) (struct) (struct :`R` 1.0 :`A` 1.0) 2.0 0.2))
  (`KismetSystemLibrary.Delay` (`self.Frequency`))
  (goto _label :!via `Open`))

(event `Open`
  (goto _label :!via `Open`))

(event `WaitForHit`
  (goto _label_4))

(event `Close`
  (goto _label :!via `Close`))