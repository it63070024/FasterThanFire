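; BP_Granade_v5 is a throwable grenade actor that breaks glass in the BreakableGlass system.
; Its Launch event throws the Granade component along player 0's camera forward with an upward lift, using a velocity-change impulse.
; It registers that component with BPBreakByObjectV6, then after a fixed delay fires the BreakByForceField breakable-glass event.
; Both break events receive the BreakOnServer flag passed to Launch.
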(event `Launch`
  (params (BreakOnServer :type "/Game/BreakableGlass_v5/Blueprints/BP_BreakOnServer_v5 Object Reference"))
  (bind (_returnvalue_x _returnvalue_y _returnvalue_z) (`KismetMathLibrary.BreakVector` (* (`self.GetActorForwardVector` (`GameplayStatics.GetPlayerCameraManager` 0)) 1500)))
  (`PrimitiveComponent.AddImpulse` (`self.Granade`) (`KismetMathLibrary.MakeVector` _returnvalue_x _returnvalue_y (+ _returnvalue_z 200.0)) "None" true)
  (`/Game/BreakableGlass_v5/Blueprints/BP_BreakByObject_v5.BreakableGlassObjectEvent` (`self.BP_BreakByObject_v6`) "ObjectTypeQuery7" (`self.Granade`) true 5.0 20.0 1.0 1.0 false BreakOnServer)
  (`KismetSystemLibrary.Delay` 5.0)
  (`/Game/BreakableGlass_v5/Blueprints/BP_BreakByForceField_v5.BreakableGlassForceFieldEvent` (`self.BreakByForceField`) "ObjectTypeQuery7" false 500.0 20.0 100.0 1000.0 5000.0 1.0 false BreakOnServer))

(fn `UserConstructionScript`)