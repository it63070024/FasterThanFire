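; Component that breaks BP_BreakableGlass_Mod panes with hit-scan line traces, given start, end, radius and impulse settings.
; Each hit pane receives a reference to the component, then breaks through BreakOnServer if multicast replication is enabled and that reference is valid, otherwise locally.
; WaitForServer and WaitForBreak add the pane to the ignore list, optionally draw a debug sphere, and retrace, letting one shot penetrate successive panes.
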(event `Again`
  (bind _as_bp_breakable_glass_v_5 (`self.As BP Breakable Glass V 5`))
  (bind _break_on_server (`self.Break on Server`))
  (bind _out_hit_location (`self.Out Hit Location`))
  (bind _outhit (`KismetSystemLibrary.LineTraceSingleForObjects` (stale `BreakableGlassHitScanEvent` Start) (stale `BreakableGlassHitScanEvent` End) (`self.CollisionObjectType`) false (`self.LastHitActor`) (stale `BreakableGlassHitScanEvent` DrawDebugType) true (stale `BreakableGlassHitScanEvent` TraceColor) (stale `BreakableGlassHitScanEvent` TraceHitColor) (stale `BreakableGlassHitScanEvent` DrawTime) :!label _label))
  (set `self.Out Hit Location` (`.Location` (`GameplayStatics.BreakHitResult` _outhit)))
  (if (== (`GameplayStatics.GetObjectClass` (`.HitActor` (`GameplayStatics.BreakHitResult` _outhit))) "/Game/BreakableGlass_v5/Blueprints/BP_BreakableGlass_Mod.BP_BreakableGlass_Mod_C")
    (bind _asbp_breakable_glass_mod (cast `/Game/BreakableGlass_v5/Blueprints/BP_BreakableGlass_Mod` (`.HitActor` (`GameplayStatics.BreakHitResult` _outhit))))
    (bind _output_get (set `self.As BP Breakable Glass V 5` _asbp_breakable_glass_mod))
    (`/Game/BreakableGlass_v5/Blueprints/BP_BreakableGlass_Mod.Set HitScan Ref` _asbp_breakable_glass_mod self)
    (if (`/Game/BreakableGlass_v5/Blueprints/BP_BreakableGlass_Mod.Replicate Multicast ( BETA )` _output_get)
      (`/Engine/EditorBlueprintResources/StandardMacros.IsValid` _break_on_server
        (:`Is Valid`
          (bind _returnvalue (* (`KismetMathLibrary.GetDirectionUnitVector` (stale `BreakableGlassHitScanEvent` Start) (stale `BreakableGlassHitScanEvent` End)) (`self.ImpulseForce`)))
          (`/Game/BreakableGlass_v5/Blueprints/BP_BreakOnServer_v5.CallBreakOnServer` _break_on_server _as_bp_breakable_glass_v_5 _out_hit_location _returnvalue (`self.AngularImpulse`) (`self.RadiusHitScan`) 0.0 1.0 1000000.0 "NewEnumerator0"))
        (:`Is Not Valid`
          (`/Game/BreakableGlass_v5/Blueprints/BP_BreakableGlass_Mod.HIT LOCAL` _as_bp_breakable_glass_v_5 _out_hit_location _returnvalue (`self.AngularImpulse`) (`self.RadiusHitScan`) 0.0 1.0 1000000.0 "NewEnumerator0" :!label _label_2)))
      (else
        (goto _label_2)))))

(event `BreakableGlassHitScanEvent`
  (params (BreakableGlassChannel :type "EObjectTypeQuery Enum" :default "ObjectTypeQuery7") (Start :type "Vector Structure") (End :type "Vector Structure") (RadiusHitScan :type "Float (double-precision)" :default 20.0) (ImpulseForce :type "Float (double-precision)" :default 1000.0) (AngularImpulse :type "Float (double-precision)" :default 1.0) (DrawDebugType :type "EDrawDebugTrace Enum" :default "None") (TraceColor :type "LinearColor Structure" :default (struct :`G` 1.0 :`A` 1.0)) (TraceHitColor :type "LinearColor Structure" :default (struct :`R` 1.0 :`A` 1.0)) (DrawTime :type "Float (double-precision)" :default 5.0) (BreakOnServer :type "/Game/BreakableGlass_v5/Blueprints/BP_BreakOnServer_v5 Object Reference"))
  (set `self.CollisionObjectType` (`|MakeArray` BreakableGlassChannel))
  (set `self.RadiusHitScan` RadiusHitScan)
  (set `self.ImpulseForce` ImpulseForce)
  (set `self.AngularImpulse` AngularImpulse)
  (set `self.Break on Server` BreakOnServer)
  (`KismetArrayLibrary.Array_Clear` (`self.LastHitActor`))
  (`KismetArrayLibrary.Array_Add` (`self.LastHitActor`) (`self.GetOwner`))
  (goto _label))

(event `WaitForServer`
  (`KismetArrayLibrary.Array_Add` (`self.LastHitActor`) (`self.As BP Breakable Glass V 5`) :!label _label_3)
  (if (`|EnumInequality` (stale `BreakableGlassHitScanEvent` DrawDebugType))
    (`KismetSystemLibrary.DrawDebugSphere` (`self.Out Hit Location`) (`self.RadiusHitScan`) 16 (stale `BreakableGlassHitScanEvent` TraceHitColor) (stale `BreakableGlassHitScanEvent` DrawTime) 0.2))
  (`self.Again`))

(event `WaitForBreak`
  (goto _label_3))