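; BP_Stone_v5 is a thrown stone projectile that can break glass and destroys itself five seconds after launch.
; Launch applies random spin and a camera-forward impulse with upward lift, then passes the stone and BreakOnServer flag to BPBreakByObject.
; An unused non-physics alternative predicts the projectile path and has the recursive MoveActor step through its points by timestamp, but that setup chain is never executed.
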(event `MoveActor`
  (bind _array_element_location (`self.Array Element Location`))
  ;[1 1 1] No Physics movement
  (if (> (`BlueprintMapLibrary.Map_Length` _array_element_location) 0)
    (bind _values (`BlueprintMapLibrary.Map_Values` _array_element_location))
    (bind (_indexofminvalue _minvalue) (`KismetMathLibrary.MinOfFloatArray` _values))
    (`KismetSystemLibrary.Delay` (- _minvalue (`self.Min Value`)))
    (bind _keys (`BlueprintMapLibrary.Map_Keys` _array_element_location))
    (bind _output (`|GetArrayItem` _keys _indexofminvalue))
    (`self.K2_SetActorLocation` _output)
    (`BlueprintMapLibrary.Map_Remove` (`self.Array Element Location`) _output)
    (set `self.LastPos` _output)
    (set `self.Min Value` _minvalue)
    (`self.MoveActor`)))

(event `Launch`
  (params (BreakOnServer :type "/Game/BreakableGlass_v5/Blueprints/BP_BreakOnServer_v5 Object Reference"))
  (bind _stone (`self.Stone`))
  (bind (_returnvalue_x _returnvalue_y _returnvalue_z) (`KismetMathLibrary.BreakVector` (* (`self.GetActorForwardVector` (`GameplayStatics.GetPlayerCameraManager` 0)) 1500)))
  (`PrimitiveComponent.AddAngularImpulseInDegrees` _stone (* (`KismetMathLibrary.RandomUnitVector`) 2000) "None" false)
  (`PrimitiveComponent.AddImpulse` _stone (`KismetMathLibrary.MakeVector` _returnvalue_x _returnvalue_y (+ _returnvalue_z 500.0)) "None" true)
  (`/Game/BreakableGlass_v5/Blueprints/BP_BreakByObject_v5.BreakableGlassObjectEvent` (`self.BP_BreakByObject`) "ObjectTypeQuery7" (`self.Stone`) true 5.0 20.0 1.0 1.0 false BreakOnServer)
  (`KismetSystemLibrary.Delay` 5.0)
  (`self.K2_DestroyActor`))

(fn `UserConstructionScript`)