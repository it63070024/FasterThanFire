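; Server relay for breakable glass that forwards break requests and wait-for-server signals between impact sources and the glass.
; CallBreakOnServer passes the hit location, impulse settings, object size and velocity, and collision type to the target's HITMULTICAST, with itself as the Server reference.
; Separate events call WaitForServer on hit scan, object, character, force field and melee instances after a validity check.
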(event `CallBreakOnServer`
  (params (Target :type "/Game/BreakableGlass_v5/Blueprints/BP_BreakableGlass_v5 Object Reference") (`Hit Location` :type "Vector Structure") (`Impulse Strength` :type "Vector Structure") (`Angular Strength` :type "Float (double-precision)") (`Impulse Radius` :type "Float (double-precision)") (`Object Half Height` :type "Float (double-precision)") (`Object Bounds` :type "Float (double-precision)") (`Object Velocity` :type "Float (double-precision)") (`Collision Type` :type "/Game/BreakableGlass_v5/Blueprints/CollisionType_Enum Enum" :default "NewEnumerator0"))
  (`/Game/BreakableGlass_v5/Blueprints/BP_BreakableGlass_v5.HIT MULTICAST` Target `Hit Location` `Impulse Strength` `Angular Strength` `Impulse Radius` `Object Half Height` `Object Bounds` `Object Velocity` `Collision Type` self))

(event `Wait for Server HitScan`
  (params (HitScan :type "/Game/BreakableGlass_v5/Blueprints/BP_BreakByHitScan_v5 Object Reference"))
  (`/Engine/EditorBlueprintResources/StandardMacros.IsValid` HitScan
    (:`Is Valid`
      (`/Game/BreakableGlass_v5/Blueprints/BP_BreakByHitScan_v5.WaitForServer` HitScan))))

(event `Wait for Server Object`
  (params (Object :type "/Game/BreakableGlass_v5/Blueprints/BP_BreakByObject_v5 Object Reference"))
  (`/Engine/EditorBlueprintResources/StandardMacros.IsValid` Object
    (:`Is Valid`
      (`/Game/BreakableGlass_v5/Blueprints/BP_BreakByObject_v5.Wait For Server` Object))))

(event `Wait For Server Character`
  (params (Character :type "/Game/BreakableGlass_v5/Blueprints/BP_BreakByCharacter_v5 Object Reference"))
  (`/Engine/EditorBlueprintResources/StandardMacros.IsValid` Character
    (:`Is Valid`
      (`/Game/BreakableGlass_v5/Blueprints/BP_BreakByCharacter_v5.WaitForServer` Character))))

(event `Wait for Server ForceField`
  (params (ForceField :type "/Game/BreakableGlass_v5/Blueprints/BP_BreakByForceField_v5 Object Reference"))
  (`/Engine/EditorBlueprintResources/StandardMacros.IsValid` ForceField
    (:`Is Valid`
      (`/Game/BreakableGlass_v5/Blueprints/BP_BreakByForceField_v5.WaitForServer` ForceField))))

(event `Wait for Server Melee`
  (params (Melee :type "/Game/BreakableGlass_v5/Blueprints/BP_BreakByMelee_v5 Object Reference"))
  (`/Engine/EditorBlueprintResources/StandardMacros.IsValid` Melee
    (:`Is Valid`
      (`/Game/BreakableGlass_v5/Blueprints/BP_BreakByMelee_v5.WaitForServer` Melee))))